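; BP_HarlowGameState is the game state for Harlow's Wallpaper and provides access to the level's single Harlow player pawn.
; GetHarlowPlayer finds the BP_HarlowPawn on first request, caches it and returns it, searching again only if the cached reference is invalid.
; A helper prints a debug message when the level holds zero or several pawns, without stopping the lookup from taking the first array entry.
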(event EventBeginPlay)

(event EventTick
  (params (DeltaSeconds :type Float%20%28single-precision%29)))

(fn ConstructionScript)

(fn GetHarlowPlayer
  (Utilities|FlowControl|Sequence
    (:then_0
      ;[0.3659 0.4963 1] Get the HarlowPlayer if not already cached
      (Utilities|IsValid (Variables|References|GetHarlowPlayer)
        (:Is%20Not%20Valid
          (bind _outactors (Actor|GetAllActorsOfClass "/Game/HarlowsWallpaper/Player/BP_HarlowPawn.BP_HarlowPawn_C"))
          (|Makesurethereis1player _outactors)
          (Variables|References|SetHarlowPlayer (Utilities|Array|Get(acopy) _outactors)))))
    (:then_1
      (return (Variables|References|GetHarlowPlayer)))))