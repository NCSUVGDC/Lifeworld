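; Day 1 spawner that places the sink handle pickup in a random unopened container once enough drawers have been opened.
; BeginPlay maps BP_HandleSpawnLocation actors to containers by tag, then runs a demo loop triggering random open events until the handle spawns.
; Subscribe functions bind drawer and door open delegates; each container event records unique opens, with both bookcase doors marked together.
; Once the drawer threshold is met, it spawns a BP_SnapperDefault with the SinkHandle mesh and tag.
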(event Custom|Drawer5
  (bind _allcontainers (Variables|Default|GetAllContainers))
  ;[1 1 1] Adds container to Opened array the first time it is opened
  (Utilities|Array|AddUnique (Variables|Default|GetOpened) "Drawer5")
  (if (not (Variables|Default|GetSpawned))
    ;[1 1 1] Checks to see if 4 or more drawers have been opened and changes 4DrawersOpen accordingly
    (for _array_element (Variables|Default|GetOpened)
      (if (Utilities|Array|ContainsItem (Variables|Default|GetDrawers) _array_element)
        (bind _result (Math|Integer|IncrementInt (Variables|Default|GetDrawersOpened))
          (:%20%20
            (if (>= _result 3)
              (Variables|Default|Set3DrawersOpen true))))))
    (if (Variables|Default|Get3DrawersOpen)
      ;[1 1 1] Select random unopened container
      (bind _output_get (Variables|Default|SetRandomContainer (Utilities|Array|Get(acopy) _allcontainers (Math|Random|RandomInteger (Utilities|Array|Length _allcontainers))) :!label _label))
      (if (Utilities|Array|ContainsItem (Variables|Default|GetOpened) _output_get)
        (goto _label)
        (else
          ;[1 1 1] Spawn object in chosen container
          (bind _returnvalue (Game|SpawnActorfromClass "/Game/HarlowsWallpaper/Interaction/Interactable_Snappers/BP_SnapperDefault.BP_SnapperDefault_C" (Math|Transform|MakeTransform (Utilities|Array|Get(acopy) (Variables|Default|GetAllLocations) (Utilities|Array|FindItem (Variables|Default|GetAllContainers) (Variables|Default|GetRandomContainer))) "0, 0, 0" "1,1,1") "AlwaysSpawn" 0 0))
          (Components|StaticMesh|SetStaticMesh (Variables|/Game/HarlowsWallpaper/Interaction/Interactable_Snappers/BP_SnapperDefault.BP_SnapperDefault_C|GetItemMeshComponent _returnvalue) "/Game/Geometry/Meshes/SinkHandle.SinkHandle")
          (Variables|Default|SetSpawned true)
          (Variables|/Script/Engine.Actor|SetTags _returnvalue (Utilities|Array|MakeArray "SinkHandle")))))))

(event Custom|Drawer4
  (bind _allcontainers (Variables|Default|GetAllContainers))
  ;[1 1 1] Adds container to Opened array the first time it is opened
  (Utilities|Array|AddUnique (Variables|Default|GetOpened) "Drawer4")
  (if (not (Variables|Default|GetSpawned))
    ;[1 1 1] Checks to see if 4 or more drawers have been opened and changes 4DrawersOpen accordingly
    (for _array_element (Variables|Default|GetOpened)
      (if (Utilities|Array|ContainsItem (Variables|Default|GetDrawers) _array_element)
        (bind _result (Math|Integer|IncrementInt (Variables|Default|GetDrawersOpened))
          (:%20%20
            (if (>= _result 3)
              (Variables|Default|Set3DrawersOpen true))))))
    (if (Variables|Default|Get3DrawersOpen)
      ;[1 1 1] Select random unopened container
      (bind _output_get (Variables|Default|SetRandomContainer (Utilities|Array|Get(acopy) _allcontainers (Math|Random|RandomInteger (Utilities|Array|Length _allcontainers))) :!label _label))
      (if (Utilities|Array|ContainsItem (Variables|Default|GetOpened) _output_get)
        (goto _label)
        (else
          ;[1 1 1] Spawn object in chosen container
          (bind _returnvalue (Game|SpawnActorfromClass "/Game/HarlowsWallpaper/Interaction/Interactable_Snappers/BP_SnapperDefault.BP_SnapperDefault_C" (Math|Transform|MakeTransform (Utilities|Array|Get(acopy) (Variables|Default|GetAllLocations) (Utilities|Array|FindItem (Variables|Default|GetAllContainers) (Variables|Default|GetRandomContainer))) "0, 0, 0" "1,1,1") "AlwaysSpawn" 0 0))
          (Components|StaticMesh|SetStaticMesh (Variables|/Game/HarlowsWallpaper/Interaction/Interactable_Snappers/BP_SnapperDefault.BP_SnapperDefault_C|GetItemMeshComponent _returnvalue) "/Game/Geometry/Meshes/SinkHandle.SinkHandle")
          (Variables|Default|SetSpawned true)
          (Variables|/Script/Engine.Actor|SetTags _returnvalue (Utilities|Array|MakeArray "SinkHandle")))))))

(event Custom|Drawer0
  (bind _allcontainers (Variables|Default|GetAllContainers))
  ;[1 1 1] Adds container to Opened array the first time it is opened
  (Utilities|Array|AddUnique (Variables|Default|GetOpened) "Drawer0")
  (if (not (Variables|Default|GetSpawned))
    ;[1 1 1] Checks to see if 4 or more drawers have been opened and changes 4DrawersOpen accordingly
    (for _array_element (Variables|Default|GetOpened)
      (if (Utilities|Array|ContainsItem (Variables|Default|GetDrawers) _array_element)
        (bind _result (Math|Integer|IncrementInt (Variables|Default|GetDrawersOpened))
          (:%20%20
            (if (>= _result 3)
              (Variables|Default|Set3DrawersOpen true))))))
    (if (Variables|Default|Get3DrawersOpen)
      ;[1 1 1] Select random unopened container
      (bind _output_get (Variables|Default|SetRandomContainer (Utilities|Array|Get(acopy) _allcontainers (Math|Random|RandomInteger (Utilities|Array|Length _allcontainers))) :!label _label))
      (if (Utilities|Array|ContainsItem (Variables|Default|GetOpened) _output_get)
        (goto _label)
        (else
          ;[1 1 1] Spawn object in chosen container
          (bind _returnvalue (Game|SpawnActorfromClass "/Game/HarlowsWallpaper/Interaction/Interactable_Snappers/BP_SnapperDefault.BP_SnapperDefault_C" (Math|Transform|MakeTransform (Utilities|Array|Get(acopy) (Variables|Default|GetAllLocations) (Utilities|Array|FindItem (Variables|Default|GetAllContainers) (Variables|Default|GetRandomContainer))) "0, 0, 0" "1,1,1") "AlwaysSpawn" 0 0))
          (Components|StaticMesh|SetStaticMesh (Variables|/Game/HarlowsWallpaper/Interaction/Interactable_Snappers/BP_SnapperDefault.BP_SnapperDefault_C|GetItemMeshComponent _returnvalue) "/Game/Geometry/Meshes/SinkHandle.SinkHandle")
          (Variables|Default|SetSpawned true)
          (Variables|/Script/Engine.Actor|SetTags _returnvalue (Utilities|Array|MakeArray "SinkHandle")))))))

(event Custom|Drawer2
  (bind _allcontainers (Variables|Default|GetAllContainers))
  ;[1 1 1] Adds container to Opened array the first time it is opened
  (Utilities|Array|AddUnique (Variables|Default|GetOpened) "Drawer2")
  (if (not (Variables|Default|GetSpawned))
    ;[1 1 1] Checks to see if 4 or more drawers have been opened and changes 4DrawersOpen accordingly
    (for _array_element (Variables|Default|GetOpened)
      (if (Utilities|Array|ContainsItem (Variables|Default|GetDrawers) _array_element)
        (bind _result (Math|Integer|IncrementInt (Variables|Default|GetDrawersOpened))
          (:%20%20
            (if (>= _result 3)
              (Variables|Default|Set3DrawersOpen true))))))
    (if (Variables|Default|Get3DrawersOpen)
      ;[1 1 1] Select random unopened container
      (bind _output_get (Variables|Default|SetRandomContainer (Utilities|Array|Get(acopy) _allcontainers (Math|Random|RandomInteger (Utilities|Array|Length _allcontainers))) :!label _label))
      (if (Utilities|Array|ContainsItem (Variables|Default|GetOpened) _output_get)
        (goto _label)
        (else
          ;[1 1 1] Spawn object in chosen container
          (bind _returnvalue (Game|SpawnActorfromClass "/Game/HarlowsWallpaper/Interaction/Interactable_Snappers/BP_SnapperDefault.BP_SnapperDefault_C" (Math|Transform|MakeTransform (Utilities|Array|Get(acopy) (Variables|Default|GetAllLocations) (Utilities|Array|FindItem (Variables|Default|GetAllContainers) (Variables|Default|GetRandomContainer))) "0, 0, 0" "1,1,1") "AlwaysSpawn" 0 0))
          (Components|StaticMesh|SetStaticMesh (Variables|/Game/HarlowsWallpaper/Interaction/Interactable_Snappers/BP_SnapperDefault.BP_SnapperDefault_C|GetItemMeshComponent _returnvalue) "/Game/Geometry/Meshes/SinkHandle.SinkHandle")
          (Variables|Default|SetSpawned true)
          (Variables|/Script/Engine.Actor|SetTags _returnvalue (Utilities|Array|MakeArray "SinkHandle")))))))

(event Custom|Drawer3
  (bind _allcontainers (Variables|Default|GetAllContainers))
  ;[1 1 1] Adds container to Opened array the first time it is opened
  (Utilities|Array|AddUnique (Variables|Default|GetOpened) "Drawer3")
  (if (not (Variables|Default|GetSpawned))
    ;[1 1 1] Checks to see if 4 or more drawers have been opened and changes 4DrawersOpen accordingly
    (for _array_element (Variables|Default|GetOpened)
      (if (Utilities|Array|ContainsItem (Variables|Default|GetDrawers) _array_element)
        (bind _result (Math|Integer|IncrementInt (Variables|Default|GetDrawersOpened))
          (:%20%20
            (if (>= _result 3)
              (Variables|Default|Set3DrawersOpen true))))))
    (if (Variables|Default|Get3DrawersOpen)
      ;[1 1 1] Select random unopened container
      (bind _output_get (Variables|Default|SetRandomContainer (Utilities|Array|Get(acopy) _allcontainers (Math|Random|RandomInteger (Utilities|Array|Length _allcontainers))) :!label _label))
      (if (Utilities|Array|ContainsItem (Variables|Default|GetOpened) _output_get)
        (goto _label)
        (else
          ;[1 1 1] Spawn object in chosen container
          (bind _returnvalue (Game|SpawnActorfromClass "/Game/HarlowsWallpaper/Interaction/Interactable_Snappers/BP_SnapperDefault.BP_SnapperDefault_C" (Math|Transform|MakeTransform (Utilities|Array|Get(acopy) (Variables|Default|GetAllLocations) (Utilities|Array|FindItem (Variables|Default|GetAllContainers) (Variables|Default|GetRandomContainer))) "0, 0, 0" "1,1,1") "AlwaysSpawn" 0 0))
          (Components|StaticMesh|SetStaticMesh (Variables|/Game/HarlowsWallpaper/Interaction/Interactable_Snappers/BP_SnapperDefault.BP_SnapperDefault_C|GetItemMeshComponent _returnvalue) "/Game/Geometry/Meshes/SinkHandle.SinkHandle")
          (Variables|Default|SetSpawned true)
          (Variables|/Script/Engine.Actor|SetTags _returnvalue (Utilities|Array|MakeArray "SinkHandle")))))))

(event Custom|BookcaseRight
  (bind _allcontainers (Variables|Default|GetAllContainers))
  ;[1 1 1] Adds container to Opened array the first time it is opened
  (Utilities|Array|AddUnique (Variables|Default|GetOpened) "BookcaseLeft")
  (Utilities|Array|AddUnique (Variables|Default|GetOpened) "BookcaseRight")
  (if (not (Variables|Default|GetSpawned))
    ;[1 1 1] Checks to see if 4 or more drawers have been opened and changes 4DrawersOpen accordingly
    (for _array_element (Variables|Default|GetOpened)
      (if (Utilities|Array|ContainsItem (Variables|Default|GetDrawers) _array_element)
        (bind _result (Math|Integer|IncrementInt (Variables|Default|GetDrawersOpened))
          (:%20%20
            (if (>= _result 3)
              (Variables|Default|Set3DrawersOpen true))))))
    (if (Variables|Default|Get3DrawersOpen)
      ;[1 1 1] Select random unopened container
      (bind _output_get (Variables|Default|SetRandomContainer (Utilities|Array|Get(acopy) _allcontainers (Math|Random|RandomInteger (Utilities|Array|Length _allcontainers))) :!label _label))
      (if (Utilities|Array|ContainsItem (Variables|Default|GetOpened) _output_get)
        (goto _label)
        (else
          ;[1 1 1] Spawn object in chosen container
          (bind _returnvalue (Game|SpawnActorfromClass "/Game/HarlowsWallpaper/Interaction/Interactable_Snappers/BP_SnapperDefault.BP_SnapperDefault_C" (Math|Transform|MakeTransform (Utilities|Array|Get(acopy) (Variables|Default|GetAllLocations) (Utilities|Array|FindItem (Variables|Default|GetAllContainers) (Variables|Default|GetRandomContainer))) "0, 0, 0" "1,1,1") "AlwaysSpawn" 0 0))
          (Components|StaticMesh|SetStaticMesh (Variables|/Game/HarlowsWallpaper/Interaction/Interactable_Snappers/BP_SnapperDefault.BP_SnapperDefault_C|GetItemMeshComponent _returnvalue) "/Game/Geometry/Meshes/SinkHandle.SinkHandle")
          (Variables|Default|SetSpawned true)
          (Variables|/Script/Engine.Actor|SetTags _returnvalue (Utilities|Array|MakeArray "SinkHandle")))))))

(event Custom|BookcaseLeft
  (bind _allcontainers (Variables|Default|GetAllContainers))
  ;[1 1 1] Adds container to Opened array the first time it is opened
  (Utilities|Array|AddUnique (Variables|Default|GetOpened) "BookcaseLeft")
  (Utilities|Array|AddUnique (Variables|Default|GetOpened) "BookcaseRight")
  (if (not (Variables|Default|GetSpawned))
    ;[1 1 1] Checks to see if 4 or more drawers have been opened and changes 4DrawersOpen accordingly
    (for _array_element (Variables|Default|GetOpened)
      (if (Utilities|Array|ContainsItem (Variables|Default|GetDrawers) _array_element)
        (bind _result (Math|Integer|IncrementInt (Variables|Default|GetDrawersOpened))
          (:%20%20
            (if (>= _result 3)
              (Variables|Default|Set3DrawersOpen true))))))
    (if (Variables|Default|Get3DrawersOpen)
      ;[1 1 1] Select random unopened container
      (bind _output_get (Variables|Default|SetRandomContainer (Utilities|Array|Get(acopy) _allcontainers (Math|Random|RandomInteger (Utilities|Array|Length _allcontainers))) :!label _label))
      (if (Utilities|Array|ContainsItem (Variables|Default|GetOpened) _output_get)
        (goto _label)
        (else
          ;[1 1 1] Spawn object in chosen container
          (bind _returnvalue (Game|SpawnActorfromClass "/Game/HarlowsWallpaper/Interaction/Interactable_Snappers/BP_SnapperDefault.BP_SnapperDefault_C" (Math|Transform|MakeTransform (Utilities|Array|Get(acopy) (Variables|Default|GetAllLocations) (Utilities|Array|FindItem (Variables|Default|GetAllContainers) (Variables|Default|GetRandomContainer))) "0, 0, 0" "1,1,1") "AlwaysSpawn" 0 0))
          (Components|StaticMesh|SetStaticMesh (Variables|/Game/HarlowsWallpaper/Interaction/Interactable_Snappers/BP_SnapperDefault.BP_SnapperDefault_C|GetItemMeshComponent _returnvalue) "/Game/Geometry/Meshes/SinkHandle.SinkHandle")
          (Variables|Default|SetSpawned true)
          (Variables|/Script/Engine.Actor|SetTags _returnvalue (Utilities|Array|MakeArray "SinkHandle")))))))

(event Custom|Cabinet
  (bind _allcontainers (Variables|Default|GetAllContainers))
  ;[1 1 1] Adds container to Opened array the first time it is opened
  (Utilities|Array|AddUnique (Variables|Default|GetOpened) "Cabinet")
  (if (not (Variables|Default|GetSpawned))
    ;[1 1 1] Checks to see if 4 or more drawers have been opened and changes 4DrawersOpen accordingly
    (for _array_element (Variables|Default|GetOpened)
      (if (Utilities|Array|ContainsItem (Variables|Default|GetDrawers) _array_element)
        (bind _result (Math|Integer|IncrementInt (Variables|Default|GetDrawersOpened))
          (:%20%20
            (if (>= _result 3)
              (Variables|Default|Set3DrawersOpen true))))))
    (if (Variables|Default|Get3DrawersOpen)
      ;[1 1 1] Select random unopened container
      (bind _output_get (Variables|Default|SetRandomContainer (Utilities|Array|Get(acopy) _allcontainers (Math|Random|RandomInteger (Utilities|Array|Length _allcontainers))) :!label _label))
      (if (Utilities|Array|ContainsItem (Variables|Default|GetOpened) _output_get)
        (goto _label)
        (else
          ;[1 1 1] Spawn object in chosen container
          (bind _returnvalue (Game|SpawnActorfromClass "/Game/HarlowsWallpaper/Interaction/Interactable_Snappers/BP_SnapperDefault.BP_SnapperDefault_C" (Math|Transform|MakeTransform (Utilities|Array|Get(acopy) (Variables|Default|GetAllLocations) (Utilities|Array|FindItem (Variables|Default|GetAllContainers) (Variables|Default|GetRandomContainer))) "0, 0, 0" "1,1,1") "AlwaysSpawn" 0 0))
          (Components|StaticMesh|SetStaticMesh (Variables|/Game/HarlowsWallpaper/Interaction/Interactable_Snappers/BP_SnapperDefault.BP_SnapperDefault_C|GetItemMeshComponent _returnvalue) "/Game/Geometry/Meshes/SinkHandle.SinkHandle")
          (Variables|Default|SetSpawned true)
          (Variables|/Script/Engine.Actor|SetTags _returnvalue (Utilities|Array|MakeArray "SinkHandle")))))))

(event Custom|Drawer6
  (bind _allcontainers (Variables|Default|GetAllContainers))
  ;[1 1 1] Adds container to Opened array the first time it is opened
  (Utilities|Array|AddUnique (Variables|Default|GetOpened) "Drawer6")
  (if (not (Variables|Default|GetSpawned))
    ;[1 1 1] Checks to see if 4 or more drawers have been opened and changes 4DrawersOpen accordingly
    (for _array_element (Variables|Default|GetOpened)
      (if (Utilities|Array|ContainsItem (Variables|Default|GetDrawers) _array_element)
        (bind _result (Math|Integer|IncrementInt (Variables|Default|GetDrawersOpened))
          (:%20%20
            (if (>= _result 3)
              (Variables|Default|Set3DrawersOpen true))))))
    (if (Variables|Default|Get3DrawersOpen)
      ;[1 1 1] Select random unopened container
      (bind _output_get (Variables|Default|SetRandomContainer (Utilities|Array|Get(acopy) _allcontainers (Math|Random|RandomInteger (Utilities|Array|Length _allcontainers))) :!label _label))
      (if (Utilities|Array|ContainsItem (Variables|Default|GetOpened) _output_get)
        (goto _label)
        (else
          ;[1 1 1] Spawn object in chosen container
          (bind _returnvalue (Game|SpawnActorfromClass "/Game/HarlowsWallpaper/Interaction/Interactable_Snappers/BP_SnapperDefault.BP_SnapperDefault_C" (Math|Transform|MakeTransform (Utilities|Array|Get(acopy) (Variables|Default|GetAllLocations) (Utilities|Array|FindItem (Variables|Default|GetAllContainers) (Variables|Default|GetRandomContainer))) "0, 0, 0" "1,1,1") "AlwaysSpawn" 0 0))
          (Components|StaticMesh|SetStaticMesh (Variables|/Game/HarlowsWallpaper/Interaction/Interactable_Snappers/BP_SnapperDefault.BP_SnapperDefault_C|GetItemMeshComponent _returnvalue) "/Game/Geometry/Meshes/SinkHandle.SinkHandle")
          (Variables|Default|SetSpawned true)
          (Variables|/Script/Engine.Actor|SetTags _returnvalue (Utilities|Array|MakeArray "SinkHandle")))))))

(event Custom|Drawer7
  (bind _allcontainers (Variables|Default|GetAllContainers))
  ;[1 1 1] Adds container to Opened array the first time it is opened
  (Utilities|Array|AddUnique (Variables|Default|GetOpened) "Drawer7")
  (if (not (Variables|Default|GetSpawned))
    ;[1 1 1] Checks to see if 4 or more drawers have been opened and changes 4DrawersOpen accordingly
    (for _array_element (Variables|Default|GetOpened)
      (if (Utilities|Array|ContainsItem (Variables|Default|GetDrawers) _array_element)
        (bind _result (Math|Integer|IncrementInt (Variables|Default|GetDrawersOpened))
          (:%20%20
            (if (>= _result 3)
              (Variables|Default|Set3DrawersOpen true))))))
    (if (Variables|Default|Get3DrawersOpen)
      ;[1 1 1] Select random unopened container
      (bind _output_get (Variables|Default|SetRandomContainer (Utilities|Array|Get(acopy) _allcontainers (Math|Random|RandomInteger (Utilities|Array|Length _allcontainers))) :!label _label))
      (if (Utilities|Array|ContainsItem (Variables|Default|GetOpened) _output_get)
        (goto _label)
        (else
          ;[1 1 1] Spawn object in chosen container
          (bind _returnvalue (Game|SpawnActorfromClass "/Game/HarlowsWallpaper/Interaction/Interactable_Snappers/BP_SnapperDefault.BP_SnapperDefault_C" (Math|Transform|MakeTransform (Utilities|Array|Get(acopy) (Variables|Default|GetAllLocations) (Utilities|Array|FindItem (Variables|Default|GetAllContainers) (Variables|Default|GetRandomContainer))) "0, 0, 0" "1,1,1") "AlwaysSpawn" 0 0))
          (Components|StaticMesh|SetStaticMesh (Variables|/Game/HarlowsWallpaper/Interaction/Interactable_Snappers/BP_SnapperDefault.BP_SnapperDefault_C|GetItemMeshComponent _returnvalue) "/Game/Geometry/Meshes/SinkHandle.SinkHandle")
          (Variables|Default|SetSpawned true)
          (Variables|/Script/Engine.Actor|SetTags _returnvalue (Utilities|Array|MakeArray "SinkHandle")))))))

(event Custom|Drawer8
  (bind _allcontainers (Variables|Default|GetAllContainers))
  ;[1 1 1] Adds container to Opened array the first time it is opened
  (Utilities|Array|AddUnique (Variables|Default|GetOpened) "Drawer8")
  (if (not (Variables|Default|GetSpawned))
    ;[1 1 1] Checks to see if 4 or more drawers have been opened and changes 4DrawersOpen accordingly
    (for _array_element (Variables|Default|GetOpened)
      (if (Utilities|Array|ContainsItem (Variables|Default|GetDrawers) _array_element)
        (bind _result (Math|Integer|IncrementInt (Variables|Default|GetDrawersOpened))
          (:%20%20
            (if (>= _result 3)
              (Variables|Default|Set3DrawersOpen true))))))
    (if (Variables|Default|Get3DrawersOpen)
      ;[1 1 1] Select random unopened container
      (bind _output_get (Variables|Default|SetRandomContainer (Utilities|Array|Get(acopy) _allcontainers (Math|Random|RandomInteger (Utilities|Array|Length _allcontainers))) :!label _label))
      (if (Utilities|Array|ContainsItem (Variables|Default|GetOpened) _output_get)
        (goto _label)
        (else
          ;[1 1 1] Spawn object in chosen container
          (bind _returnvalue (Game|SpawnActorfromClass "/Game/HarlowsWallpaper/Interaction/Interactable_Snappers/BP_SnapperDefault.BP_SnapperDefault_C" (Math|Transform|MakeTransform (Utilities|Array|Get(acopy) (Variables|Default|GetAllLocations) (Utilities|Array|FindItem (Variables|Default|GetAllContainers) (Variables|Default|GetRandomContainer))) "0, 0, 0" "1,1,1") "AlwaysSpawn" 0 0))
          (Components|StaticMesh|SetStaticMesh (Variables|/Game/HarlowsWallpaper/Interaction/Interactable_Snappers/BP_SnapperDefault.BP_SnapperDefault_C|GetItemMeshComponent _returnvalue) "/Game/Geometry/Meshes/SinkHandle.SinkHandle")
          (Variables|Default|SetSpawned true)
          (Variables|/Script/Engine.Actor|SetTags _returnvalue (Utilities|Array|MakeArray "SinkHandle")))))))

(event Custom|Drawer1
  (bind _allcontainers (Variables|Default|GetAllContainers))
  ;[1 1 1] Adds container to Opened array the first time it is opened
  (Utilities|Array|AddUnique (Variables|Default|GetOpened) "Drawer1")
  (if (not (Variables|Default|GetSpawned))
    ;[1 1 1] Checks to see if 4 or more drawers have been opened and changes 4DrawersOpen accordingly
    (for _array_element (Variables|Default|GetOpened)
      (if (Utilities|Array|ContainsItem (Variables|Default|GetDrawers) _array_element)
        (bind _result (Math|Integer|IncrementInt (Variables|Default|GetDrawersOpened))
          (:%20%20
            (if (>= _result 3)
              (Variables|Default|Set3DrawersOpen true))))))
    (if (Variables|Default|Get3DrawersOpen)
      ;[1 1 1] Select random unopened container
      (bind _output_get (Variables|Default|SetRandomContainer (Utilities|Array|Get(acopy) _allcontainers (Math|Random|RandomInteger (Utilities|Array|Length _allcontainers))) :!label _label))
      (if (Utilities|Array|ContainsItem (Variables|Default|GetOpened) _output_get)
        (goto _label)
        (else
          ;[1 1 1] Spawn object in chosen container
          (bind _returnvalue (Game|SpawnActorfromClass "/Game/HarlowsWallpaper/Interaction/Interactable_Snappers/BP_SnapperDefault.BP_SnapperDefault_C" (Math|Transform|MakeTransform (Utilities|Array|Get(acopy) (Variables|Default|GetAllLocations) (Utilities|Array|FindItem (Variables|Default|GetAllContainers) (Variables|Default|GetRandomContainer))) "0, 0, 0" "1,1,1") "AlwaysSpawn" 0 0))
          (Components|StaticMesh|SetStaticMesh (Variables|/Game/HarlowsWallpaper/Interaction/Interactable_Snappers/BP_SnapperDefault.BP_SnapperDefault_C|GetItemMeshComponent _returnvalue) "/Game/Geometry/Meshes/SinkHandle.SinkHandle")
          (Variables|Default|SetSpawned true)
          (Variables|/Script/Engine.Actor|SetTags _returnvalue (Utilities|Array|MakeArray "SinkHandle")))))))

(event EventBeginPlay
  (bind _allcontainers (Variables|Default|GetAllContainers))
  (Utilities|FlowControl|Delay 0.2)
  ;[1 1 1] Get Container Spawning Locations
  (bind _outactors (Actor|GetAllActorsOfClass "/Game/HarlowsWallpaper/DayBPs/Day1/BP_HandleSpawnLocation.BP_HandleSpawnLocation_C"))
  (for _array_element _outactors
    (Utilities|Array|SetArrayElem (Variables|Default|GetAllLocations) (Utilities|Array|FindItem (Variables|Default|GetAllContainers) (Utilities|Array|Get(acopy) (Variables|/Script/Engine.Actor|GetTags _array_element))) (.location (Transformation|GetActorTransform _array_element)) true))
  ;[1 1 1] Demo: Open random containers until object spawns
  (bind _output_get (Variables|Default|SetDemoContainer (Utilities|Array|Get(acopy) _allcontainers (Math|Random|RandomInteger (Utilities|Array|Length _allcontainers))) :!label _label))
  (switch name _output_get
    (:Drawer0
      (CallFunction|Drawer0))
    (:Drawer1
      (CallFunction|Drawer1))
    (:Drawer2
      (CallFunction|Drawer2))
    (:Drawer3
      (CallFunction|Drawer3))
    (:Drawer4
      (CallFunction|Drawer4))
    (:Drawer5
      (CallFunction|Drawer5))
    (:Drawer6
      (CallFunction|Drawer6))
    (:Drawer7
      (CallFunction|Drawer7))
    (:Drawer8
      (CallFunction|Drawer8))
    (:BookcaseRight
      (CallFunction|BookcaseRight))
    (:BookcaseLeft
      (CallFunction|BookcaseLeft))
    (:Cabinet
      (CallFunction|Cabinet)))
  (if (not (Variables|Default|GetSpawned))
    (Utilities|FlowControl|Delay 3.0)
    (goto _label)))

(fn ConstructionScript)

(fn SubscribetoDrawer
  (params (Drawer :type BP%20Drawer%20Hole%20Object%20Reference))
  (bind _asbp_drawer_physics (Utilities|Casting|CastToBP_DrawerPhysics (Variables|/Script/Engine.ChildActorComponent|GetChildActor (Variables|/Game/HarlowsWallpaper/Interaction/Interactable_Dresser/BP_DrawerHole.BP_DrawerHole_C|GetDefaultDrawer Drawer))))
  (Variables|Default|SetDrawer _asbp_drawer_physics)
  (switch int (Variables|/Game/HarlowsWallpaper/Interaction/Interactable_Dresser/BP_DrawerHole.BP_DrawerHole_C|GetDrawerID Drawer)
    (:0
      (EventDispatchers|BindEventtoDrawerOpened (Variables|Default|GetDrawer) (EventDispatchers|CreateEvent :!event Custom|Drawer0)))
    (:1
      (EventDispatchers|BindEventtoDrawerOpened (Variables|Default|GetDrawer) (EventDispatchers|CreateEvent :!event Custom|Drawer1)))
    (:2
      (EventDispatchers|BindEventtoDrawerOpened (Variables|Default|GetDrawer) (EventDispatchers|CreateEvent :!event Custom|Drawer2)))
    (:3
      (EventDispatchers|BindEventtoDrawerOpened (Variables|Default|GetDrawer) (EventDispatchers|CreateEvent :!event Custom|Drawer3)))
    (:4
      (EventDispatchers|BindEventtoDrawerOpened (Variables|Default|GetDrawer) (EventDispatchers|CreateEvent :!event Custom|Drawer4)))
    (:5
      (EventDispatchers|BindEventtoDrawerOpened (Variables|Default|GetDrawer) (EventDispatchers|CreateEvent :!event Custom|Drawer5)))
    (:6
      (EventDispatchers|BindEventtoDrawerOpened (Variables|Default|GetDrawer) (EventDispatchers|CreateEvent :!event Custom|Drawer6)))
    (:7
      (EventDispatchers|BindEventtoDrawerOpened (Variables|Default|GetDrawer) (EventDispatchers|CreateEvent :!event Custom|Drawer7)))
    (:8
      (EventDispatchers|BindEventtoDrawerOpened (Variables|Default|GetDrawer) (EventDispatchers|CreateEvent :!event Custom|Drawer8)))))

(fn SubscribetoRightDoor
  (params (Door :type BP%20Door%20Object%20Reference))
  (Variables|Default|SetDoorReference Door)
  (EventDispatchers|BindEventtoDoorOpened (Variables|Default|GetDoorReference) (EventDispatchers|CreateEvent :!event Custom|BookcaseRight)))

(fn SubscribetoLeftDoor
  (params (Door :type BP%20Door%20Object%20Reference))
  (Variables|Default|SetDoorReference Door)
  (EventDispatchers|BindEventtoDoorOpened (Variables|Default|GetDoorReference) (EventDispatchers|CreateEvent :!event Custom|BookcaseLeft)))

(fn SubscribetoCabinet
  (params (Door :type BP%20Door%20Object%20Reference))
  (Variables|Default|SetDoorReference Door)
  (EventDispatchers|BindEventtoDoorOpened (Variables|Default|GetDoorReference) (EventDispatchers|CreateEvent :!event Custom|Cabinet)))