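; Grabbable malfunctioning flip clock for Day 4: plugging it in cycles the minutes; unplugging freezes them and signals Receiver if they match RequiredMins.
; Plug snap events toggle DemoMode, which Tick uses to advance minutes after a Delay.
; Flipper animations and per-face dynamic materials' CurrentFrame parameter display the digits.
; Hour increment and TimeSystem display sync are disconnected, so hours never advance; fast clocks call StopClock five seconds after BeginPlay.
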(event Custom|FlipHrs
  (bind _hrs_flipper (Variables|Default|Gethrs_flipper))
  (bind _hrs_var (Variables|Default|Gethrs_var))
  (bind _returnvalue (Math|Conversions|ToFloat(Integer) _hrs_var))
  ;[1 1 1] Flip Hours Animation
  (Components|Animation|SetAnimation _hrs_flipper 0)
  (Components|Timeline|SetPlayRate _hrs_flipper (Variables|Default|GetAnimPlayRate)) ; override animation speed
  (Audio|Components|Audio|Play _hrs_flipper false)
  (Rendering|Material|SetScalarParameterValue (Variables|Default|GethrsBottom2_matVar) "CurrentFrame" _returnvalue :!class /Script/Engine.MaterialInstanceDynamic)
  (Utilities|FlowControl|Delay (Variables|Default|GetAnimDurationDelay)) ; time for flip animation to end
  (Rendering|Material|SetScalarParameterValue (Variables|Default|GethrsBottom_matVar) "CurrentFrame" _returnvalue :!class /Script/Engine.MaterialInstanceDynamic)
  (Components|Animation|SetAnimation (Variables|Default|Gethrs_flipper) 0))

(event Custom|FlipMins
  (bind _mins_flipper (Variables|Default|Getmins_flipper))
  (bind _mins_var (Variables|Default|Getmins_var))
  (bind _returnvalue (Math|Conversions|ToFloat(Integer) _mins_var))
  ;[1 1 1] Flip Minutes Animation
  (Components|Animation|SetAnimation _mins_flipper 0)
  (Components|Timeline|SetPlayRate _mins_flipper (Variables|Default|GetAnimPlayRate)) ; override animation speed
  (Audio|Components|Audio|Play _mins_flipper false)
  (Rendering|Material|SetScalarParameterValue (Variables|Default|GetminsBottom2_matVar) "CurrentFrame" _returnvalue :!class /Script/Engine.MaterialInstanceDynamic)
  (Utilities|FlowControl|Delay (Variables|Default|GetAnimDurationDelay)) ; time for flip animation to end
  (Rendering|Material|SetScalarParameterValue (Variables|Default|GetminsBottom_matVar) "CurrentFrame" _returnvalue :!class /Script/Engine.MaterialInstanceDynamic)
  (Components|Animation|SetAnimation (Variables|Default|Getmins_flipper) 0))

(event Custom|StopClock
  (Variables|Default|SetDemoMode false)
  (if (== (Variables|Default|GetRequiredMins) (Variables|Default|Getmins_var))
    (Default|SetFlipclock (Variables|Default|GetReceiver) true)))

(event Custom|StartClock
  (Variables|Default|SetDemoMode true)
  (Default|SetFlipclock (Variables|Default|GetReceiver) false))

(event EventBeginPlay
  (bind _plug (Variables|Default|GetPlug))
  (bind _minuteduration (Variables|Default|GetMinuteDuration))
  (bind _returnvalue (/ 1.0 _minuteduration))
  (bind _returnvalue_2 (* 2.0 _returnvalue))
  (EventDispatchers|BindEventtoSnappedNotify _plug (delegate Custom|StartClock))
  (EventDispatchers|BindEventtoUnsnappedNotify _plug (delegate Custom|StopClock))
  (Default|SetPhysicsGrab (Variables|Default|GetGrabable) (Variables|Default|Getflipclock_body) "/Game/UVRFProject/Framework/Hands/Model/Animations/Grabs/grab_round_big_2.grab_round_big_2" 25.0)
  (if (Variables|Default|GetDemoMode)
    ;[1 1 1] For demo mode, set delay to minute duration.
    (Variables|Default|SetDelay (Variables|Default|GetMinuteDuration))
    (Utilities|FlowControl|Sequence :!label _label
      (:then_0
        ;[1 1 1] First Animation to show starting time
        (CallFunction|FlipMins)
        (CallFunction|FlipHrs))
      (:then_1
        ;[1 1 1] Check for Debug Text (destroy)
        (if (Variables|Default|GetDisplayDebugText)
          ;[1 1 1] Update TextRender
          (Rendering|Components|TextRender|SetText (Variables|Default|GetTextRender) (Utilities|Text|ToText(String) (Utilities|String|Append (Utilities|String|ToString(Integer) (Variables|Default|Gethrs_var)) ":" (CallFunction|MinutesFormatting))))
          (else
            (Components|DestroyComponent (Variables|Default|GetTextRender)))))
      (:then_2
        ;[1 1 1] Define Animation PlayRate and Delays
        (if (< _minuteduration 1.21)
          (Variables|Default|SetAnimPlayRate _returnvalue_2)
          (Variables|Default|SetAnimDurationDelay (* 1.1 (/ 1.21 _returnvalue_2)))
          (Utilities|FlowControl|Delay 5.0)
          (CallFunction|StopClock))))
    (else
      ;[1 1 1] Sync TimeSystem with display rate
      (bind _outactors (Actor|GetAllActorsOfClass "/Script/Harlows_Wallpaper.TimeSystem"))
      (for _array_element _outactors
        (bind _astime_system (Utilities|Casting|CastToTimeSystem _array_element)
          (:then
            (Variables|Default|SetInGameTime _astime_system)
            (goto _label))
          (:CastFailed
            (CallFunction|PrintDebug "Error: Couldn't find TimeSystem in World" true true "NewEnumerator2" self)))))))

(event EventTick
  (params (DeltaSeconds :type Float%20%28single-precision%29))
  (if (== (Actor|GetParentActor) "/Game/UVRFProject/Framework/Hands/HandBP.HandBP")
    (Development|PrintString "Grabbed"))
  ;[1 1 1] Define Clock Speed
  (Utilities|FlowControl|Delay (Variables|Default|GetDelay))
  (Utilities|FlowControl|Sequence
    (:then_0
      ;[1 1 1] Check if running Demo Mode
      (if (Variables|Default|GetDemoMode)
        (Utilities|FlowControl|Sequence
          (:then_0
            ;[1 1 1] Increment Minutes
            (if (< (Variables|Default|Getmins_var) 59)
              (Variables|Default|Setmins_var (+ (Variables|Default|Getmins_var) 1))
              (else
                (Variables|Default|Setmins_var 0))))
          (:then_1
            (CallFunction|FlipMins)))))
    (:then_1
      ;[1 1 1] Check for Debug Text (if it exists)
      (if (Variables|Default|GetDisplayDebugText)
        ;[1 1 1] Update TextRender
        (Rendering|Components|TextRender|SetText (Variables|Default|GetTextRender) (Utilities|Text|ToText(String) (Utilities|String|Append (Utilities|String|ToString(Integer) (Variables|Default|Gethrs_var)) ":" (CallFunction|MinutesFormatting))))))))

(fn ConstructionScript
  (Utilities|FlowControl|Sequence
    (:then_0
      ;[1 1 1] Setup Top dynamic Material
      (Utilities|FlowControl|Sequence
        (:then_0
          (bind _returnvalue (Rendering|Material|CreateDynamicMaterialInstance "/Game/HarlowsWallpaper/Environment/flipclock/flipclock_face_top.flipclock_face_top" "None" :!class /Script/Engine.KismetMaterialLibrary))
          (Variables|Default|SethrsTop_matVar _returnvalue)
          (Rendering|Material|SetMaterial (Variables|Default|Gethrs_panel) 1 (Variables|Default|GethrsTop_matVar)))
        (:then_1
          (bind _returnvalue_2 (Rendering|Material|CreateDynamicMaterialInstance "/Game/HarlowsWallpaper/Environment/flipclock/flipclock_face_top.flipclock_face_top" "None" :!class /Script/Engine.KismetMaterialLibrary))
          (Variables|Default|SethrsTop2_matVar _returnvalue_2)
          (Rendering|Material|SetMaterial (Variables|Default|Gethrs_flipper) 1 (Variables|Default|GethrsTop2_matVar)))
        (:then_2
          (bind _returnvalue_3 (Rendering|Material|CreateDynamicMaterialInstance "/Game/HarlowsWallpaper/Environment/flipclock/flipclock_face_top.flipclock_face_top" "None" :!class /Script/Engine.KismetMaterialLibrary))
          (Variables|Default|SetminsTop_matVar _returnvalue_3)
          (Rendering|Material|SetMaterial (Variables|Default|Getmins_panel) 1 (Variables|Default|GetminsTop_matVar)))
        (:then_3
          (bind _returnvalue_4 (Rendering|Material|CreateDynamicMaterialInstance "/Game/HarlowsWallpaper/Environment/flipclock/flipclock_face_top.flipclock_face_top" "None" :!class /Script/Engine.KismetMaterialLibrary))
          (Variables|Default|SetminsTop2_matVar _returnvalue_4)
          (Rendering|Material|SetMaterial (Variables|Default|Getmins_flipper) 1 (Variables|Default|GetminsTop2_matVar)))))
    (:then_1
      ;[1 1 1] Setup Bottom dynamic Material
      (Utilities|FlowControl|Sequence
        (:then_0
          (bind _returnvalue_5 (Rendering|Material|CreateDynamicMaterialInstance "/Game/HarlowsWallpaper/Environment/flipclock/flipclock_face_bottom.flipclock_face_bottom" "None" :!class /Script/Engine.KismetMaterialLibrary))
          (Variables|Default|SethrsBottom_matVar _returnvalue_5)
          (Rendering|Material|SetMaterial (Variables|Default|Gethrs_panel) 0 (Variables|Default|GethrsBottom_matVar)))
        (:then_1
          (bind _returnvalue_6 (Rendering|Material|CreateDynamicMaterialInstance "/Game/HarlowsWallpaper/Environment/flipclock/flipclock_face_bottom.flipclock_face_bottom" "None" :!class /Script/Engine.KismetMaterialLibrary))
          (Variables|Default|SethrsBottom2_matVar _returnvalue_6)
          (Rendering|Material|SetMaterial (Variables|Default|Gethrs_flipper) 0 (Variables|Default|GethrsBottom2_matVar)))
        (:then_2
          (bind _returnvalue_7 (Rendering|Material|CreateDynamicMaterialInstance "/Game/HarlowsWallpaper/Environment/flipclock/flipclock_face_bottom.flipclock_face_bottom" "None" :!class /Script/Engine.KismetMaterialLibrary))
          (Variables|Default|SetminsBottom_matVar _returnvalue_7)
          (Rendering|Material|SetMaterial (Variables|Default|Getmins_panel) 0 (Variables|Default|GetminsBottom_matVar)))
        (:then_3
          (bind _returnvalue_8 (Rendering|Material|CreateDynamicMaterialInstance "/Game/HarlowsWallpaper/Environment/flipclock/flipclock_face_bottom.flipclock_face_bottom" "None" :!class /Script/Engine.KismetMaterialLibrary))
          (Variables|Default|SetminsBottom2_matVar _returnvalue_8)
          (Rendering|Material|SetMaterial (Variables|Default|Getmins_flipper) 0 (Variables|Default|GetminsBottom2_matVar)))))))

(fn MinutesFormatting
  (if (> (Variables|Default|Getmins_var) 9)
    (return (Utilities|String|ToString(Integer) (Variables|Default|Getmins_var)))
    (else
      (return (Utilities|String|Append "0" (Utilities|String|ToString(Integer) (Variables|Default|Getmins_var)))))))