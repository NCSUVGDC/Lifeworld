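; Lock Blueprint for the keys-and-locks interactables, showing either a locked or an unlocked mesh.
; The construction script calls Lock or Unlock from StartLocked, and each function toggles visibility of the two meshes.
; Both functions set IsLocked to true, so Unlock changes only the visuals.
; The Keyhole overlap event is an empty stub, so key detection does nothing here.
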(event OnComponentBeginOverlap(Keyhole)
  (params (OverlappedComponent :type Primitive%20Component%20Object%20Reference) (OtherActor :type Actor%20Object%20Reference) (OtherComp :type Primitive%20Component%20Object%20Reference) (OtherBodyIndex :type Integer) (bFromSweep :type Boolean) (SweepResult :type Hit%20Result%20Structure%20%28by%20ref%29))
  ;[0.3047 1 0.2011] Key is in keyhole
)

(event EventBeginPlay)

(event Collision|EventActorBeginOverlap
  (params (OtherActor :type Actor%20Object%20Reference)))

(event EventTick
  (params (DeltaSeconds :type Float%20%28single-precision%29)))

(fn ConstructionScript
  ;[1 1 1] Start locked/unlocked
  (if (Variables|Default|GetStartLocked)
    (CallFunction|Lock)
    (else
      (CallFunction|Unlock))))

(fn Lock
  (Variables|Default|SetisLocked true)
  ;[1 1 1] Set visible mesh
  (Rendering|SetVisibility (Variables|Default|Getlock_locked_mesh) true true)
  (Rendering|SetVisibility (Variables|Default|Getlock_unlocked_mesh) false true))

(fn Unlock
  (Variables|Default|SetisLocked true)
  ;[1 1 1] Set visible mesh
  (Rendering|SetVisibility (Variables|Default|Getlock_locked_mesh) false true)
  (Rendering|SetVisibility (Variables|Default|Getlock_unlocked_mesh) true true))