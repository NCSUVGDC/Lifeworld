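; BP_TimeReceiver tracks whether the two clocks of a clock puzzle, a flip clock and a grandfather clock, are both correct.
; SetFlipclock and SetGrandfather each store an incoming correctness flag, then check both flags together.
; The result is only a debug print, GOOD when both are correct and BAD otherwise, with no further gameplay effect in this Blueprint.
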(event Custom|SetGrandfather
  (params (Value :type Boolean))
  (bind _output_get (Variables|Default|SetGrandfatherCorrect? Value))
  (if (and (Variables|Default|GetFlipclockCorrect?) _output_get)
    (Development|PrintString "GOOD")
    (else
      (Development|PrintString "BAD"))))

(event Custom|SetFlipclock
  (params (Value :type Boolean))
  (bind _output_get (Variables|Default|SetFlipclockCorrect? Value))
  (if (and (Variables|Default|GetGrandfatherCorrect?) _output_get)
    (Development|PrintString "GOOD")
    (else
      (Development|PrintString "BAD"))))

(fn ConstructionScript)