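; BP_BasicItem is a generic grabbable item actor for Harlow's Wallpaper, configured per instance with a mesh, material and grab settings.
; The construction script applies the mesh and material and adds or removes a DrawerItem tag from a flag.
; On BeginPlay it registers the mesh with its Grabable component, using either fixed left and right grab transforms or a relative grab, both with a grab animation.
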(event Collision|EventActorBeginOverlap
  (params (OtherActor :type Actor%20Object%20Reference)))

(event EventTick
  (params (DeltaSeconds :type Float%20%28single-precision%29)))

(event EventBeginPlay
  (bind _itemmeshcomponent (Variables|Default|GetItemMeshComponent))
  (bind _grabanimation (Variables|Default|GetGrabAnimation))
  (if (Variables|Default|GetUseFixedGrab)
    (Default|SetFixedGrab (Variables|Default|GetGrabable) _itemmeshcomponent (Variables|Default|GetGrabTransformLeft) _grabanimation (Variables|Default|GetGrabTransformRight))
    (else
      (Default|SetRelativeGrab (Variables|Default|GetGrabable) _itemmeshcomponent _grabanimation))))

(fn ConstructionScript
  (bind _tags (Variables|Actor|GetTags))
  (Components|StaticMesh|SetStaticMesh (Variables|Default|GetItemMeshComponent) (Variables|Default|GetItemMesh))
  (Rendering|Material|SetMaterial (Variables|Default|GetItemMeshComponent) 0 (Variables|Default|GetItemMaterial))
  ;[1 1 1] Add/remove DrawerItem tag
  (if (Variables|Default|GetDrawerItem)
    (if (not (Utilities|Array|ContainsItem _tags "DrawerItem"))
      (Utilities|Array|Add _tags "DrawerItem"))
    (else
      (Utilities|Array|RemoveItem _tags "DrawerItem"))))