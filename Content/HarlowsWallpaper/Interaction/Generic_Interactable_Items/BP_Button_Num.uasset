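; BP_Button_Num is an interactable number button that shows a single digit on a text render and cycles it when pressed.
; An IndexCollider entering the trigger swaps the cube material to Brass and increments the number, wrapping from 9 back to 0.
; Leaving the trigger restores the Porcelain material.
; The text is set on BeginPlay and refreshed after each increment.
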(event OnComponentBeginOverlap(Trigger)
  (params (OverlappedComponent :type Primitive%20Component%20Object%20Reference) (OtherActor :type Actor%20Object%20Reference) (OtherComp :type Primitive%20Component%20Object%20Reference) (OtherBodyIndex :type Integer) (bFromSweep :type Boolean) (SweepResult :type Hit%20Result%20Structure%20%28by%20ref%29))
  (Utilities|Casting|CastToIndexCollider OtherActor)
  (Rendering|Material|SetMaterial (Variables|Default|GetCube) 0 "/Game/HarlowsWallpaper/Materials/Bronze.Brass")
  (CallFunction|IncreaseNumber))

(event OnComponentEndOverlap(Trigger)
  (params (OverlappedComponent :type Primitive%20Component%20Object%20Reference) (OtherActor :type Actor%20Object%20Reference) (OtherComp :type Primitive%20Component%20Object%20Reference) (OtherBodyIndex :type Integer))
  (Utilities|Casting|CastToIndexCollider OtherActor)
  (Rendering|Material|SetMaterial (Variables|Default|GetCube) 0 "/Game/HarlowsWallpaper/Materials/porcelain.porcelain"))

(event Custom|IncreaseNumber
  (if (== (Variables|Default|GetNumber) 9)
    (Variables|Default|SetNumber 0)
    (else
      (Math|Integer|IncrementInt (Variables|Default|GetNumber)
        (:%20%20
          _))))
  (Rendering|Components|TextRender|SetText (Variables|Default|GetTextRender) (Utilities|Text|ToText(Integer) (Variables|Default|GetNumber))))

(event EventBeginPlay
  (Rendering|Components|TextRender|SetText (Variables|Default|GetTextRender) (Utilities|Text|ToText(Integer) (Variables|Default|GetNumber))))

(event Collision|EventActorBeginOverlap
  (params (OtherActor :type Actor%20Object%20Reference)))

(event EventTick
  (params (DeltaSeconds :type Float%20%28single-precision%29)))

(fn ConstructionScript)