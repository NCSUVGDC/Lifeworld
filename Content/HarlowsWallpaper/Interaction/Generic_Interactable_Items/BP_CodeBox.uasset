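; BP_CodeBox is an interactable code box that unlocks when three number buttons show the correct code.
; Every tick it casts the three child actors to BP_Button_Num, joins their numbers into a string and compares it to Code.
; A match sets Unlocked and turns the box material green, with no relock on a later mismatch.
; A failed cast prints a debug string.
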(event EventTick
  (params (DeltaSeconds :type Float%20%28single-precision%29))
  (bind _asbp_button_num (Utilities|Casting|CastToBP_Button_Num (Variables|/Script/Engine.ChildActorComponent|GetChildActor (Variables|Default|Getbutton1)))
    (:then
      (bind _asbp_button_num_2 (Utilities|Casting|CastToBP_Button_Num (Variables|/Script/Engine.ChildActorComponent|GetChildActor (Variables|Default|Getbutton2)))
        (:then
          (bind _asbp_button_num_3 (Utilities|Casting|CastToBP_Button_Num (Variables|/Script/Engine.ChildActorComponent|GetChildActor (Variables|Default|Getbutton3)))
            (:then
              (if (Utilities|Enum|Equal(Enum) (Utilities|String|Append (Utilities|String|ToString(Integer) (Variables|/Game/HarlowsWallpaper/Interaction/Generic_Interactable_Items/BP_Button_Num.BP_Button_Num_C|GetNumber _asbp_button_num)) (Utilities|String|ToString(Integer) (Variables|/Game/HarlowsWallpaper/Interaction/Generic_Interactable_Items/BP_Button_Num.BP_Button_Num_C|GetNumber _asbp_button_num_2)) (Utilities|String|ToString(Integer) (Variables|/Game/HarlowsWallpaper/Interaction/Generic_Interactable_Items/BP_Button_Num.BP_Button_Num_C|GetNumber _asbp_button_num_3))) (Variables|Default|Getcode))
                (Variables|Default|SetUnlocked true)
                (Rendering|Material|SetMaterial (Variables|Default|Getbox) 0 "/Engine/EngineDebugMaterials/VertexColorViewMode_GreenOnly.VertexColorViewMode_GreenOnly")))
            (:CastFailed
              (Development|PrintString "BRUH!!!!!!!" true true "(R=0.000000,G=0.660000,B=1.000000,A=1.000000)" 1e+02 :!label _label))))
        (:CastFailed
          (goto _label))))
    (:CastFailed
      (goto _label))))

(fn ConstructionScript)