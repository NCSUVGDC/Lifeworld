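; BP_DestructibleItem is a generic grabbable item whose destructible mesh is set from ItemMesh in the construction script.
; On BeginPlay it configures its Grabable component for Relative, Fixed or Physics grabbing according to GrabType, using the mesh as the grab volume.
; When the mesh fractures, it clears the grab and disallows further grabbing.
; The grab-notify and overlap events are empty, and the physics-disable and damage nodes are disconnected.
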(event OnComponentFracture(ItemMeshComponent)
  (params (HitPoint :type Vector%20%28by%20ref%29 :default "0, 0, 0") (HitDirection :type Vector%20%28by%20ref%29 :default "0, 0, 0"))
  (bind _grabable (Variables|Default|GetGrabable))
  (Default|ClearGrab _grabable)
  (Variables|/Game/UVRFProject/Framework/Hands/Grabable.Grabable_C|SetGrabAllowed _grabable false))

(event GrabNotify(Grabable))

(event EventBeginPlay
  (bind _grabanimation (Variables|Default|GetGrabAnimation))
  (bind _itemmeshcomponent (Variables|Default|GetItemMeshComponent))
  (switch Utilities|FlowControl|Switch|SwitchonGrabTypes (Variables|Default|GetGrabType)
    (:NewEnumerator0
      (Default|SetRelativeGrab (Variables|Default|GetGrabable) _itemmeshcomponent _grabanimation))
    (:NewEnumerator1
      (Default|SetFixedGrab (Variables|Default|GetGrabable) _itemmeshcomponent (Variables|Default|GetGrabTransformLeft) _grabanimation (Variables|Default|GetGrabTransformRight)))
    (:NewEnumerator7
      (Default|SetPhysicsGrab (Variables|Default|GetGrabable) (Variables|Default|GetItemMeshComponent) (Variables|Default|GetGrabAnimation) (Variables|Default|GetGrabDistanceMax)))))

(event Collision|EventActorBeginOverlap
  (params (OtherActor :type Actor%20Object%20Reference)))

(fn ConstructionScript
  (Class|DestructibleComponent|SetDestructibleMesh (Variables|Default|GetItemMeshComponent) (Variables|Default|GetItemMesh)))