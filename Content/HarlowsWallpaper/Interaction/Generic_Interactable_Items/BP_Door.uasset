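; BP_Door is a grabbable physics door that swings on a hinge, can be locked, and signals opening and closing with sounds.
; The construction script applies mesh and materials, keeping only the physics constraint for a right, left or bottom hinge.
; Tick measures the swing with a 2D dot-product angle, using separate open and close thresholds to fire events.
; Tick also applies lock changes, including at startup, by toggling physics simulation and grabbing.
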(event Custom|DoorOpened_Event
  (bind _hingeloc (Variables|Default|GetHingeLoc))
  (if (Variables|Default|GetBedroomDoor?)
    (Audio|SpawnSoundAttached "/Game/HarlowsWallpaper/SoundEffects/Door/bedroomDoor/Household_Door_Closet_Door_Open_01.Household_Door_Closet_Door_Open_01" _hingeloc "None" "0, 0, 0" "0, 0, 0" "KeepRelativeOffset" false 1.0 1.0 0.0 0 0)
    (else
      (Audio|SpawnSoundAttached "/Game/HarlowsWallpaper/SoundEffects/Door/Household_Door_Cabinet_Door_Open_01_Cue.Household_Door_Cabinet_Door_Open_01_Cue" _hingeloc "None" "0, 0, 0" "0, 0, 0" "KeepRelativeOffset" false 1.0 1.0 0.0 0 0))))

(event Custom|DoorClosed_Event
  (bind _hingeloc (Variables|Default|GetHingeLoc))
  (if (Variables|Default|GetBedroomDoor?)
    (Audio|SpawnSoundAttached "/Game/HarlowsWallpaper/SoundEffects/Door/bedroomDoor/Household_Door_Closet_Door_Close_01_Cue.Household_Door_Closet_Door_Close_01_Cue" _hingeloc "None" "0, 0, 0" "0, 0, 0" "KeepRelativeOffset" false 1.0 1.0 0.0 0 0)
    (else
      (Audio|SpawnSoundAttached "/Game/HarlowsWallpaper/SoundEffects/Door/Household_Door_Cabinet_Door_Close_01_Cue.Household_Door_Cabinet_Door_Close_01_Cue" _hingeloc "None" "0, 0, 0" "0, 0, 0" "KeepRelativeOffset" false 1.0 1.0 0.9 0 0))))

(event EventBeginPlay
  (Default|SetPhysicsGrab (Variables|Default|GetGrabable) (Variables|Default|GetDoor) (Variables|DoorSetup|GetGrabAnimation) (Variables|DoorSetup|GetGrabDistanceMax)))

(event EventTick
  (params (DeltaSeconds :type Float%20%28single-precision%29))
  (bind _locked (Variables|Default|GetLocked))
  (bind _returnvalue (not _locked))
  (Utilities|FlowControl|Sequence
    (:then_0
      ;[1 1 1] Door opened and closed events
      (bind _doorangle (CallFunction|GetDoorAngle (Transformation|GetWorldLocation (Variables|Default|GetHingeLoc)) (Transformation|GetWorldLocation (Variables|Default|GetDoorPositionLoc)) (Transformation|GetWorldLocation (Variables|Default|GetDoorClosedLoc))))
      (if (Variables|Openness|GetOpened)
        (if (< (Math|Float|Absolute(Float) _doorangle) (Variables|Openness|GetCloseEventAngle)) ; Getting Closed on this Tick
          (Variables|Openness|SetOpened false)
          (CallFunction|DoorClosedEvent)
          (Default|CallDoorClosed))
        (elif (> (Math|Float|Absolute(Float) _doorangle) (Variables|Openness|GetOpenEventAngle)) ; Getting Opened on this Tick
          (Variables|Openness|SetOpened true)
          (CallFunction|DoorOpenedEvent)
          (Default|CallDoorOpened))))
    (:then_1
      ;[1 1 1] Lock/UnlockDoor
      (if (Math|Boolean|NotEqual(Boolean) (Variables|Default|GetLocked) (Variables|Default|GetPrevLocked)) ; If locked value changed this frame
        (Variables|Default|SetPrevLocked _locked)
        (Utilities|FlowControl|Sequence
          (:then_0
            (Utilities|FlowControl|DoOnce false
              (:Completed
                (if (Variables|Default|GetBedroomDoor?)
                  (for _array_element (Components|GetChildrenComponents (Variables|Default|GetSceneRoot) true)
                    (if (== (Utilities|GetClass _array_element) "/Script/Engine.StaticMeshComponent")
                      (bind _asstatic_mesh_component (Utilities|Casting|CastToStaticMeshComponent _array_element))
                      (Collision|SetCollisionResponsetoChannel _asstatic_mesh_component "ECC_PhysicsBody" "ECR_Overlap")))))))
          (:then_1
            (Physics|SetSimulatePhysics (Variables|Default|GetDoor) _returnvalue)
            (Variables|/Game/UVRFProject/Framework/Hands/Grabable.Grabable_C|SetGrabAllowed (Variables|Default|GetGrabable) _returnvalue)))))))

(fn ConstructionScript
  ;[0.9979 0.4961 1] Set up visuals
  (Components|StaticMesh|SetStaticMesh (Variables|Default|GetDoor) (Variables|Visuals|GetDoorMesh))
  (for (_array_element _array_index) (Variables|Visuals|GetMaterials)
    (Rendering|Material|SetMaterial (Variables|Default|GetDoor) _array_index _array_element))
  (Variables|Default|SetPrevLocked (not (Variables|Default|GetLocked))) ; Set to opposite of locked so it will make adjustments on startup
  ;[1 0.5279 0.3049] Set up physics constraints
  (switch Utilities|FlowControl|Switch|SwitchonDoorTypes (Variables|DoorSetup|GetDoorType)
    (:NewEnumerator0
      (Components|DestroyComponent (Variables|Default|GetBottomPhysicsConstraint))
      (Components|DestroyComponent (Variables|Default|GetLeftPhysicsConstraint))
      (Transformation|SetRelativeTransform (Variables|Default|GetOpen) (Math|Transform|MakeTransform "0, 0, 0" (Math|Rotator|MakeRotator 0.0 0.0 (- 9e+01 (Variables|Openness|GetOpenEventAngle)))) false false)
      (Class|PhysicsConstraintComponent|SetAngularSwing1Limit (Variables|Default|GetRightPhysicsConstraint) "ACM_Limited" (Variables|Default|GetDoorSwingLimit)))
    (:NewEnumerator1
      (Components|DestroyComponent (Variables|Default|GetBottomPhysicsConstraint))
      (Components|DestroyComponent (Variables|Default|GetRightPhysicsConstraint))
      (Transformation|SetRelativeTransform (Variables|Default|GetOpen) (Math|Transform|MakeTransform "0, 0, 0" (Math|Rotator|MakeRotator 0.0 0.0 (+ (Variables|Openness|GetOpenEventAngle) -9e+01))) false false)
      (Class|PhysicsConstraintComponent|SetAngularSwing1Limit (Variables|Default|GetLeftPhysicsConstraint) "ACM_Limited" (Variables|Default|GetDoorSwingLimit)))
    (:NewEnumerator2
      (Components|DestroyComponent (Variables|Default|GetLeftPhysicsConstraint))
      (Components|DestroyComponent (Variables|Default|GetRightPhysicsConstraint))
      (Transformation|SetRelativeTransform (Variables|Default|GetOpen) (Math|Transform|MakeTransform "0, 0, 0" (Math|Rotator|MakeRotator 0.0 (Variables|Openness|GetOpenEventAngle) 0.0)) false false)
      (Class|PhysicsConstraintComponent|SetAngularSwing1Limit (Variables|Default|GetBottomPhysicsConstraint) "ACM_Limited" (Variables|Default|GetDoorSwingLimit)))))

(fn GetDoorAngle
  (params (HingeLoc :type Vector) (DoorPositionLoc :type Vector) (ZeroLoc :type Vector))
  ;[1 1 1] Make two vectors. One represents the door's closed position, the other is its current postion
  (LocalVariables|Seta (Math|Vector2D|MakeVector2D (- (.x HingeLoc) (.x DoorPositionLoc)) (- (.y HingeLoc) (.y DoorPositionLoc))))
  (LocalVariables|Setb (Math|Vector2D|MakeVector2D (- (.x HingeLoc) (.x ZeroLoc)) (- (.y HingeLoc) (.y ZeroLoc))))
  ;[1 1 1] Law of cosines to find angle
  (return (Class|KismetMathLibrary|DegAcos (/ (Math|Vector2D|DotProduct(2D) (LocalVariables|Geta) (LocalVariables|Getb)) (* (Math|Vector2D|Vector2DLength (LocalVariables|Geta)) (Math|Vector2D|Vector2DLength (LocalVariables|Getb)))))))