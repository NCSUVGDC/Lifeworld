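; BP_TestDrawerEventSubscriber is a test Blueprint that shows whether a drawer's opened and closed events reach a subscriber.
; On BeginPlay it binds its handlers through the referenced Drawer's bind functions.
; The handlers swap the Sphere's material to Brass on open and Brown on close, with optional debug prints gated by PrintDebugStatements.
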(event Custom|DoorOpened_Event
  (Rendering|Material|SetMaterial (Variables|Default|GetSphere) 0 "/Game/HarlowsWallpaper/Materials/Bronze.Brass")
  (if (Variables|Default|GetPrintDebugStatements)
    (Development|PrintString "Received Door Open")))

(event Custom|DoorClosed_Event
  (Rendering|Material|SetMaterial (Variables|Default|GetSphere) 0 "/Game/HarlowsWallpaper/Materials/Brown.Brown")
  (if (Variables|Default|GetPrintDebugStatements)
    (Development|PrintString "Received Door Closed")))

(event EventBeginPlay
  (bind _drawer (Variables|Default|GetDrawer))
  (EventDispatchers|BindEventtoDrawerOpened _drawer (delegate Custom|DoorOpened_Event))
  (EventDispatchers|BindEventtoDrawerClosed _drawer (delegate Custom|DoorClosed_Event)))

(fn ConstructionScript)