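; Interactable book actor that can be grabbed, opened and paged through, showing text on left and right page widgets.
; PageFwd and PageBkwd track the page, write the matching spread from the Pages array, and wrap between closed and last spread.
; Each state change swaps physics grab volumes between closed and open boxes.
; BeginPlay starts the book closed and blank, handing its reference to the book's animation Blueprint.
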(event Custom|PageBkwd
  (bind _numpages (Variables|Default|GetNumPages))
  (bind _result (Math|Integer|DecrementInt (Variables|Default|GetCurPage))
    (:%20%20
      (if (< _result 0)
        (Variables|Default|SetOpen? true)
        (Variables|Default|SetCurPage _numpages)
        (Variables|Default|SetCurText (- (* _numpages 2) 2))
        (CallFunction|ChangeTexts)
        (Default|ClearGrab (Variables|Default|GetClosedGrab))
        (Default|SetPhysicsGrab (Variables|Default|GetOpenGrab) (Variables|Default|GetOpenBox) "/Game/UVRFProject/Framework/Hands/Model/Animations/Grabs/grab_round_big.grab_round_big" 25.0)
        (elif (== (Variables|Default|GetCurPage) 0)
          (Variables|Default|SetOpen? false)
          (CallFunction|ClearTexts)
          (Variables|Default|SetCurText -1)
          (Default|ClearGrab (Variables|Default|GetOpenGrab))
          (Default|SetPhysicsGrab (Variables|Default|GetClosedGrab) (Variables|Default|GetClosedBox) "/Game/UVRFProject/Framework/Hands/Model/Animations/Grabs/grab_round_big.grab_round_big" 25.0)
          (else
            (Variables|Default|SetCurText (- (Variables|Default|GetCurText) 3))
            (CallFunction|ChangeTexts)
            (Default|ClearGrab (Variables|Default|GetClosedGrab))
            (Default|SetPhysicsGrab (Variables|Default|GetOpenGrab) (Variables|Default|GetOpenBox) "/Game/UVRFProject/Framework/Hands/Model/Animations/Grabs/grab_round_big.grab_round_big" 25.0)))))))

(event Custom|PageFwd
  (bind _result (Math|Integer|IncrementInt (Variables|Default|GetCurPage))
    (:%20%20
      (if (> _result (Variables|Default|GetNumPages))
        (Variables|Default|SetOpen? false)
        (Variables|Default|SetCurPage 0)
        (CallFunction|ClearTexts)
        (Variables|Default|SetCurText -1)
        (Default|ClearGrab (Variables|Default|GetOpenGrab))
        (Default|SetPhysicsGrab (Variables|Default|GetClosedGrab) (Variables|Default|GetClosedBox) "/Game/UVRFProject/Framework/Hands/Model/Animations/Grabs/grab_round_big.grab_round_big" 25.0)
        (else
          (Variables|Default|SetOpen? true)
          (Math|Integer|IncrementInt (Variables|Default|GetCurText)
            (:%20%20
              (CallFunction|ChangeTexts)
              (Default|ClearGrab (Variables|Default|GetClosedGrab))
              (Default|SetPhysicsGrab (Variables|Default|GetOpenGrab) (Variables|Default|GetOpenBox) "/Game/UVRFProject/Framework/Hands/Model/Animations/Grabs/grab_round_big.grab_round_big" 25.0))))))))

(event Custom|ClearTexts
  (bind _asw_book_page (Utilities|Casting|CastToW_BookPage (UserInterface|GetUserWidgetObject (Variables|Default|GetLeftPage))))
  (Rendering|Components|TextRender|SetText (Variables|/Game/HarlowsWallpaper/Interaction/Interactable_Book/W_BookPage.W_BookPage_C|GetText _asw_book_page) "")
  (bind _asw_book_page_2 (Utilities|Casting|CastToW_BookPage (UserInterface|GetUserWidgetObject (Variables|Default|GetRightPage))))
  (Rendering|Components|TextRender|SetText (Variables|/Game/HarlowsWallpaper/Interaction/Interactable_Book/W_BookPage.W_BookPage_C|GetText _asw_book_page_2) ""))

(event Custom|ChangeTexts
  (if true
    (bind _asw_book_page (Utilities|Casting|CastToW_BookPage (UserInterface|GetUserWidgetObject (Variables|Default|GetLeftPage))))
    (Rendering|Components|TextRender|SetText (Variables|/Game/HarlowsWallpaper/Interaction/Interactable_Book/W_BookPage.W_BookPage_C|GetText _asw_book_page) (Utilities|Array|Get(acopy) (Variables|Default|GetPages) (Variables|Default|GetCurText))))
  (Math|Integer|IncrementInt (Variables|Default|GetCurText)
    (:%20%20
      (if true
        (bind _asw_book_page_2 (Utilities|Casting|CastToW_BookPage (UserInterface|GetUserWidgetObject (Variables|Default|GetRightPage))))
        (Rendering|Components|TextRender|SetText (Variables|/Game/HarlowsWallpaper/Interaction/Interactable_Book/W_BookPage.W_BookPage_C|GetText _asw_book_page_2) (Utilities|Array|Get(acopy) (Variables|Default|GetPages) (Variables|Default|GetCurText)))))))

(event EventBeginPlay
  (Default|SetPhysicsGrab (Variables|Default|GetClosedGrab) (Variables|Default|GetClosedBox) "/Game/UVRFProject/Framework/Hands/Model/Animations/Grabs/grab_round_big.grab_round_big" 25.0)
  (CallFunction|ClearTexts)
  (Variables|Default|SetCurText -1)
  (bind _asbook_anim_bp (Utilities|Casting|CastToBook_Anim_BP (Components|SkeletalMesh|GetAnimInstance (Variables|Default|GetBook))))
  (Variables|/Game/HarlowsWallpaper/Environment/book/Book_Anim_BP.Book_Anim_BP_C|SetBookActor _asbook_anim_bp self)
  (Utilities|FlowControl|Delay 5.0))

(fn ConstructionScript)