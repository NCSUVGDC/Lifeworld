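; BP_PageTurn is a grabbable cube handle on a BP_BasicBook that turns its pages forward or back.
; TurnPageDir sets its side; overlapping that side's book trigger, checked on begin and end overlap, calls PageFwd or PageBkwd, with a LastTurner name check against repeats.
; After a turn or release, it spawns an attached replacement at the side's resting offset, registers it with the book and destroys itself.
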(event GrabNotify(Grabable)
  (Rendering|Material|SetMaterial (Variables|Default|GetCube) 0 "/Game/UVRFProject/Framework/Buttons/3DButtonBorderMat.3DButtonBorderMat"))

(event ReleaseNotify(Grabable)
  (CallFunction|ResetTurners))

(event Custom|ResetTurners
  (bind _book (Variables|Default|GetBook))
  (bind _book_2 (Variables|Default|GetBook))
  (switch int (Variables|Default|GetTurnPageDir?)
    (:-1
      (bind _returnvalue (Game|SpawnActorfromClass "BP_PageTurn_C" (Math|Transform|MakeTransform "-20.000000, 0,10.000000" "0, 0, 0" (Variables|Default|GetTurnerScale)) "Undefined" _book_2 0))
      (Transformation|AttachActorToActor _returnvalue _book_2 "None" "KeepRelative" "KeepRelative" "KeepRelative" true)
      (Variables|/Game/HarlowsWallpaper/Interaction/Interactable_Book/BP_BasicBook.BP_BasicBook_C|SetTurnPageLeft _book_2 _returnvalue)
      (Variables|BP_PageTurn_C|SetTurnPageDir? _returnvalue -1))
    (:1
      (bind _returnvalue_2 (Game|SpawnActorfromClass "BP_PageTurn_C" (Math|Transform|MakeTransform "20.000000, 0,10.000000" "0, 0, 0" (Variables|Default|GetTurnerScale)) "Undefined" _book 0))
      (Transformation|AttachActorToActor _returnvalue_2 _book "None" "KeepRelative" "KeepRelative" "KeepRelative" true)
      (Variables|/Game/HarlowsWallpaper/Interaction/Interactable_Book/BP_BasicBook.BP_BasicBook_C|SetTurnPageRight _book _returnvalue_2)
      (Variables|BP_PageTurn_C|SetTurnPageDir? _returnvalue_2 1)))
  (Actor|DestroyActor))

(event EventBeginPlay
  (Default|SetRelativeGrab (Variables|Default|GetGrabable) (Variables|Default|GetCube) "/Game/UVRFProject/Framework/Hands/Model/Animations/Grabs/grab_thin.grab_thin")
  (bind _asbp_basic_book (Utilities|Casting|CastToBP_BasicBook (Components|GetOwner)))
  (Variables|Default|SetBook _asbp_basic_book)
  (switch int (Variables|Default|GetTurnPageDir?)
    (:-1
      (Variables|Default|SetTransform (Math|Transform|MakeTransform "-20.000000, 0,10.000000" "0, 0, 0" (Variables|Default|GetTurnerScale))))
    (:1
      (Variables|Default|SetTransform (Math|Transform|MakeTransform "20.000000, 0,10.000000" "0, 0, 0" (Variables|Default|GetTurnerScale))))))

(event Collision|EventActorEndOverlap
  (params (OtherActor :type Actor%20Object%20Reference))
  (switch int (Variables|Default|GetTurnPageDir?)
    (:-1
      (if (Class|PrimitiveComponent|IsOverlappingComponent (Variables|Default|GetCube) (Variables|/Game/HarlowsWallpaper/Interaction/Interactable_Book/BP_BasicBook.BP_BasicBook_C|GetLeftTrigger (Variables|Default|GetBook)))
        (if (Utilities|Enum|NotEqual(Enum) (Utilities|GetDisplayName self) (Variables|Default|GetLastTurner))
          (Variables|Default|SetLastTurner (Utilities|GetDisplayName self))
          (Rendering|Material|SetMaterial (Variables|Default|GetCube) 0 "/Game/HarlowsWallpaper/Materials/Bronze.Brass")
          (Default|PageFwd (Variables|Default|GetBook))
          (CallFunction|ResetTurners :!label _label))))
    (:1
      (if (Class|PrimitiveComponent|IsOverlappingComponent (Variables|Default|GetCube) (Variables|/Game/HarlowsWallpaper/Interaction/Interactable_Book/BP_BasicBook.BP_BasicBook_C|GetRightTrigger (Variables|Default|GetBook)))
        (if (Utilities|Enum|NotEqual(Enum) (Utilities|GetDisplayName self) (Variables|Default|GetLastTurner))
          (Variables|Default|SetLastTurner (Utilities|GetDisplayName self))
          (Rendering|Material|SetMaterial (Variables|Default|GetCube) 0 "/Game/HarlowsWallpaper/Materials/Bronze.Brass")
          (Default|PageBkwd (Variables|Default|GetBook))
          (goto _label))))))

(event Collision|EventActorBeginOverlap
  (params (OtherActor :type Actor%20Object%20Reference))
  (switch int (Variables|Default|GetTurnPageDir?)
    (:-1
      (if (Class|PrimitiveComponent|IsOverlappingComponent (Variables|Default|GetCube) (Variables|/Game/HarlowsWallpaper/Interaction/Interactable_Book/BP_BasicBook.BP_BasicBook_C|GetLeftTrigger (Variables|Default|GetBook)))
        (if (Utilities|Enum|NotEqual(Enum) (Utilities|GetDisplayName self) (Variables|Default|GetLastTurner))
          (Variables|Default|SetLastTurner (Utilities|GetDisplayName self))
          (Rendering|Material|SetMaterial (Variables|Default|GetCube) 0 "/Game/HarlowsWallpaper/Materials/Bronze.Brass")
          (Default|PageFwd (Variables|Default|GetBook))
          (CallFunction|ResetTurners :!label _label))))
    (:1
      (if (Class|PrimitiveComponent|IsOverlappingComponent (Variables|Default|GetCube) (Variables|/Game/HarlowsWallpaper/Interaction/Interactable_Book/BP_BasicBook.BP_BasicBook_C|GetRightTrigger (Variables|Default|GetBook)))
        (if (Utilities|Enum|NotEqual(Enum) (Utilities|GetDisplayName self) (Variables|Default|GetLastTurner))
          (Variables|Default|SetLastTurner (Utilities|GetDisplayName self))
          (Rendering|Material|SetMaterial (Variables|Default|GetCube) 0 "/Game/HarlowsWallpaper/Materials/Bronze.Brass")
          (Default|PageBkwd (Variables|Default|GetBook))
          (goto _label))))))

(fn ConstructionScript)