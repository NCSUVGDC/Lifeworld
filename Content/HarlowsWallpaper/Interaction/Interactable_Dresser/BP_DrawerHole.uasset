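; Dresser slot that lets a hand-held BP_DresserDrawer be inserted, slid and pulled out, starting with its default drawer fully in.
; An aligned, held drawer overlapping the open hole snaps in, attaches and loses physics and gravity.
; A Tick state machine restricts Grabable axes to sliding along X, switching state by distance thresholds.
; Removal restores physics and snaps to the hold position, with the drawer's held objects briefly made static during snaps.
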(event OnComponentBeginOverlap(DresserHole)
  (params (OverlappedComponent :type Primitive%20Component%20Object%20Reference) (OtherActor :type Actor%20Object%20Reference) (OtherComp :type Primitive%20Component%20Object%20Reference) (OtherBodyIndex :type Integer) (bFromSweep :type Boolean) (SweepResult :type Hit%20Result%20Structure%20%28by%20ref%29))
  ;[0.3047 1 0.2011] Key is in keyhole
  (if (and (Components|ComponentHasTag OtherComp "DresserInsert") (Variables|Default|GetDresserHoleOpen)) ; Overlapped with back of dresser drawer and is accepting drawers
    (bind _asbp_dresser_drawer (Utilities|Casting|CastToBP_DresserDrawer OtherActor))
    (Utilities|IsValid (Variables|/Game/UVRFProject/Framework/Hands/Grabable.Grabable_C|GetHand (Variables|/Game/HarlowsWallpaper/Interaction/Interactable_Dresser/BP_DresserDrawer.BP_DresserDrawer_C|GetGrabable _asbp_dresser_drawer)) ; If it is being held. (Throwing drawer into hole doesn't make sense)
      (:Is%20Valid
        (Variables|Default|SetDresserDrawer _asbp_dresser_drawer)
        ;[0.1415 0.1413 1] Check if key is aligned correctly to be in hole
        (if (Math|Rotator|Equal(Rotator) (.rotation (Class|KismetMathLibrary|ConvertTransformtoRelative (Transformation|GetActorTransform (Variables|Default|GetDresserDrawer)) (Transformation|GetActorTransform self))) "0, 0, 0" (Variables|Default|GetDresserInsertRotTolerance)) ; If key is rightside up (within tolerance)
          (CallFunction|SnapDrawertoInsertPos)
          (Variables|Default|SetDresserHoleState "NewEnumerator0")
          (Variables|Default|SetAreProperAxesRestricted false)
          (Variables|Default|SetDresserHoleOpen false))))))

(event EventBeginPlay
  ;[1 0.1865 0.7445] Set Default drawer as inserted
  (bind _asbp_dresser_drawer (Utilities|Casting|CastToBP_DresserDrawer (Variables|/Script/Engine.ChildActorComponent|GetChildActor (Variables|Default|GetDefaultDrawer))))
  (Variables|Default|SetDresserDrawer _asbp_dresser_drawer)
  (Variables|Default|SetDresserHoleOpen false)
  (Variables|Default|SetDrawerGravityEnabled true)
  (Variables|Default|SetDrawerSimulationPhysics true)
  (Variables|Default|SetAreProperAxesRestricted false)
  (Variables|Default|SetDresserHoleState "NewEnumerator1"))

(event Collision|EventActorBeginOverlap
  (params (OtherActor :type Actor%20Object%20Reference)))

(event EventTick
  (params (DeltaSeconds :type Float%20%28single-precision%29))
  (Utilities|IsValid (Variables|Default|GetDresserDrawer)
    (:Is%20Valid
      (if (Variables|Default|GetAreHeldObjectsStatic)
        (Default|SetHeldObjectsStatic (Variables|Default|GetDresserDrawer) false)
        (Variables|Default|SetAreHeldObjectsStatic false))
      (switch Utilities|FlowControl|Switch|SwitchonDresserHoleStates (Variables|Default|GetDresserHoleState)
        (:NewEnumerator2
          (CallFunction|NoDrawerTick))
        (:NewEnumerator0
          (CallFunction|DrawerInsertedTick))
        (:NewEnumerator1
          (CallFunction|DrawerPushedinTick))))))

(fn ConstructionScript)

(fn SnapDrawertoInsertPos
  (bind _dresserdrawer (Variables|Default|GetDresserDrawer))
  (bind _dresserdrawer_2 (Variables|Default|GetDresserDrawer))
  (bind _dresserdrawer_3 (Variables|Default|GetDresserDrawer))
  (bind _grabable (Variables|/Game/HarlowsWallpaper/Interaction/Interactable_Dresser/BP_DresserDrawer.BP_DresserDrawer_C|GetGrabable _dresserdrawer))
  (bind _drawer (Variables|/Game/HarlowsWallpaper/Interaction/Interactable_Dresser/BP_DresserDrawer.BP_DresserDrawer_C|GetDrawer _dresserdrawer_2))
  (Default|SetHeldObjectsStatic (Variables|Default|GetDresserDrawer) true)
  (Variables|Default|SetAreHeldObjectsStatic true)
  (Transformation|AttachActorToActor _dresserdrawer_3 self "None" "KeepWorld" "KeepWorld" "KeepWorld" false)
  (Transformation|SetActorRelativeTransform _dresserdrawer_3 (Variables|Default|GetDrawerSnapPoint) false true)
  ;[1 0.9952 0.3837] Turn off gravity and physics while in hole, turn them on when not.
  (Variables|Default|SetDrawerGravityEnabled (Variables|/Game/UVRFProject/Framework/Hands/Grabable.Grabable_C|GetGravityEnabled _grabable))
  (Variables|/Game/UVRFProject/Framework/Hands/Grabable.Grabable_C|SetGravityEnabled _grabable false)
  (Variables|Default|SetDrawerSimulationPhysics (Variables|/Game/UVRFProject/Framework/Hands/Grabable.Grabable_C|GetSimulationPhysics _grabable))
  (Variables|/Game/UVRFProject/Framework/Hands/Grabable.Grabable_C|SetSimulationPhysics _grabable false)
  (Physics|SetSimulatePhysics _drawer false)
  (Physics|SetEnableGravity _drawer false))

(fn NoDrawerTick)

(fn DrawerInsertedTick
  (bind _dresserdrawer (Variables|Default|GetDresserDrawer))
  (bind _rootcomponent (Variables|/Script/Engine.Actor|GetRootComponent _dresserdrawer))
  (bind _returnvalue (Transformation|GetRelativeTransform _rootcomponent))
  (if (Variables|Default|GetAreProperAxesRestricted)
    _
    (else
      (Default|SetRestrictedAxes (Variables|/Game/HarlowsWallpaper/Interaction/Interactable_Dresser/BP_DresserDrawer.BP_DresserDrawer_C|GetGrabable (Variables|Default|GetDresserDrawer)) false false true true true true true true true true true true)
      (Variables|Default|SetAreProperAxesRestricted true)))
  ;[0.2868 1 0.9701] Check if leaving state
  (if (>= (.x (.location _returnvalue)) (Variables|DrawerDistances|GetDrawerInsertedPullOutDistance)) ; if pulled out
    (Variables|Default|SetDresserHoleState "NewEnumerator2")
    (Variables|Default|SetAreProperAxesRestricted false)
    (CallFunction|RemoveDrawer)
    (elif (<= (.x (.location _returnvalue)) (Variables|DrawerDistances|GetDrawerFullyInsertedDistance)) ; If pushed all the way in
      (Variables|Default|SetDresserHoleState "NewEnumerator1")
      (Variables|Default|SetAreProperAxesRestricted false)
      (Transformation|SetActorRelativeLocation (Variables|Default|GetDresserDrawer) (Math|Vector|MakeVector (Variables|DrawerDistances|GetDrawerFullyInsertedDistance) (.y (.location _returnvalue)) (.z (.location _returnvalue)))))))

(fn DrawerPushedinTick
  (bind _dresserdrawer (Variables|Default|GetDresserDrawer))
  (bind _rootcomponent (Variables|/Script/Engine.Actor|GetRootComponent _dresserdrawer))
  (bind _returnvalue (Transformation|GetRelativeTransform _rootcomponent))
  (if (Variables|Default|GetAreProperAxesRestricted)
    _
    (else
      (Default|SetRestrictedAxes (Variables|/Game/HarlowsWallpaper/Interaction/Interactable_Dresser/BP_DresserDrawer.BP_DresserDrawer_C|GetGrabable (Variables|Default|GetDresserDrawer)) false true true true true true true true true true true true)
      (Variables|Default|SetAreProperAxesRestricted true)
      (Transformation|SetActorRelativeLocation (Variables|Default|GetDresserDrawer) (Math|Vector|MakeVector (Variables|DrawerDistances|GetDrawerFullyInsertedDistance) (.y (.location _returnvalue)) (.z (.location _returnvalue))))))
  ;[0.2868 1 0.9701] Check if leaving state
  (if (>= (.x (.location (Transformation|GetRelativeTransform (Variables|/Script/Engine.Actor|GetRootComponent (Variables|Default|GetDresserDrawer))))) (Variables|DrawerDistances|GetFullInsertionPullOutDistance)) ; if pulled out
    (Variables|Default|SetDresserHoleState "NewEnumerator0")
    (Variables|Default|SetAreProperAxesRestricted false)))

(fn RemoveDrawer
  (bind _dresserdrawer (Variables|Default|GetDresserDrawer))
  (bind _grabable (Variables|/Game/HarlowsWallpaper/Interaction/Interactable_Dresser/BP_DresserDrawer.BP_DresserDrawer_C|GetGrabable _dresserdrawer))
  (Development|PrintString "Removing Drawer")
  (if (== (Transformation|GetAttachParent (Variables|/Script/Engine.Actor|GetRootComponent _dresserdrawer)) self)
    (Transformation|DetachFromActor "KeepWorld" "KeepWorld" "KeepWorld"))
  (Variables|Default|SetDresserHoleOpen true)
  (Default|SetRestrictedAxes _grabable false false false false false false false false false false false false)
  (Utilities|IsValid (Variables|/Game/UVRFProject/Framework/Hands/Grabable.Grabable_C|GetHand _grabable) ; Do not call snap if the key is not held
    (:Is%20Valid
      _)
    (:Is%20Not%20Valid
      _))
  (Variables|/Game/UVRFProject/Framework/Hands/Grabable.Grabable_C|SetGravityEnabled _grabable (Variables|Default|GetDrawerGravityEnabled))
  (Variables|/Game/UVRFProject/Framework/Hands/Grabable.Grabable_C|SetSimulationPhysics _grabable (Variables|Default|GetDrawerSimulationPhysics))
  (Default|SetHeldObjectsStatic (Variables|Default|GetDresserDrawer) true)
  (Default|SnaptoHoldPos _grabable)
  (Variables|Default|SetAreHeldObjectsStatic true))