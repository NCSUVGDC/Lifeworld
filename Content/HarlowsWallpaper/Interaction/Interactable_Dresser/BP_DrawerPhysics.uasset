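; Physics-driven dresser drawer that the player grabs through several grab zones, optionally limited to the handle by destroying the others.
; BeginPlay configures the Grabable component and offsets the physics constraint's reference position.
; Tick measures the distance between two reference points, firing opened and closed events at separate thresholds.
; A helper attaches tagged items inside HoldItemZone to the drawer actor, or detaches them and re-enables physics.
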(event EventBeginPlay
  (Default|SetPhysicsGrab (Variables|Default|GetGrabable) (Variables|Default|GetDrawer) "/Game/UVRFProject/Framework/Hands/Model/Animations/Grabs/grab_thick_obj.grab_thick_obj" (Variables|Default|GetGrabDistanceMax))
  (Variables|Default|SetLastLocation (Transformation|GetWorldTransform (Variables|Default|GetDrawer)))
  (Class|PhysicsConstraintComponent|SetConstraintReferencePosition (Variables|Default|GetPhysicsConstraint) "Frame2" (Math|Vector|MakeVector -15.0 0.0 0.0)))

(event Collision|EventActorBeginOverlap
  (params (OtherActor :type Actor%20Object%20Reference)))

(event EventTick
  (params (DeltaSeconds :type Float%20%28single-precision%29))
  ;[1 1 1] Drawer opened and closed events
  (bind _opendistance (CallFunction|GetDrawerOpenDistance))
  (if (Variables|Default|GetOpened)
    (if (< (Math|Float|Absolute(Float) _opendistance) (Variables|Default|GetCloseEventDistance)) ; Getting Closed on this Tick
      (Variables|Default|SetOpened false)
      (Default|CallDrawerClosed))
    (elif (> (Math|Float|Absolute(Float) _opendistance) (Variables|Default|GetOpenEventDistance)) ; Getting Opened on this Tick
      (Variables|Default|SetOpened true)
      (Default|CallDrawerOpened))))

(fn ConstructionScript
  (bind _debugmode (Variables|Default|GetDebugMode))
  (bind _output_get (Variables|/Game/UVRFProject/Framework/Hands/Grabable.Grabable_C|SetGrabZones (Variables|Default|GetGrabable) (Utilities|Array|MakeArray (Variables|Default|GetGrabZone0) (Variables|Default|GetGrabZone1) (Variables|Default|GetGrabZone2) (Variables|Default|GetGrabZone3) (Variables|Default|GetGrabZone4) (Variables|Default|GetHandleGrabZone))))
  (for _array_element _output_get
    (Rendering|SetVisibility _array_element _debugmode false))
  (Rendering|SetVisibility (Variables|Default|GetHoldItemZone) _debugmode false))

(fn SetHeldObjectsStatic
  (params (IsStatic :type Boolean))
  (for _array_element (Collision|GetOverlappingActors (Variables|Default|GetHoldItemZone) 0 :!class /Script/Engine.PrimitiveComponent)
    (if (Actor|ActorHasTag _array_element "DrawerItem")
      (if IsStatic
        (Transformation|AttachActorToActor _array_element self "None" "KeepWorld" "KeepWorld" "KeepWorld" true)
        (else
          (Transformation|DetachFromActor _array_element "KeepWorld" "KeepWorld" "KeepWorld")
          (bind _asprimitive_component (Utilities|Casting|CastToPrimitiveComponent (Variables|/Script/Engine.Actor|GetRootComponent _array_element)))
          (Physics|SetSimulatePhysics _asprimitive_component true))))))

(fn MakeOnlyGrabbablebyHandle
  (Components|DestroyComponent (Variables|Default|GetGrabZone0))
  (Components|DestroyComponent (Variables|Default|GetGrabZone1))
  (Components|DestroyComponent (Variables|Default|GetGrabZone2))
  (Components|DestroyComponent (Variables|Default|GetGrabZone3))
  (Components|DestroyComponent (Variables|Default|GetGrabZone4)))

(fn GetDrawerOpenDistance
  (return (Math|Float|Absolute(Float) (Math|Vector|VectorLength (- (Transformation|GetWorldLocation (Variables|Default|GetClosedRef)) (Transformation|GetWorldLocation (Variables|Default|GetOpenRef)))))))