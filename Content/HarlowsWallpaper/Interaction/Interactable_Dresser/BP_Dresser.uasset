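; BP_Dresser is an interactable dresser built from nine drawer-hole child actors that hold physics drawers.
; Its construction script copies the dresser-level DrawersRemovable setting into each BP_DrawerHole.
; GetDrawers walks the child actor components down to each hole's default drawer and returns the collected BP_DrawerPhysics references.
; The event graph holds no logic.
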(event EventBeginPlay)

(event Collision|EventActorBeginOverlap
  (params (OtherActor :type Actor%20Object%20Reference)))

(event EventTick
  (params (DeltaSeconds :type Float%20%28single-precision%29)))

(fn ConstructionScript
  (Utilities|SetDrawerDefaults (Variables|Default|GetDresserHole0))
  (Utilities|SetDrawerDefaults (Variables|Default|GetDresserHole1))
  (Utilities|SetDrawerDefaults (Variables|Default|GetDresserHole3))
  (Utilities|SetDrawerDefaults (Variables|Default|GetDresserHole4))
  (Utilities|SetDrawerDefaults (Variables|Default|GetDresserHole5))
  (Utilities|SetDrawerDefaults (Variables|Default|GetDresserHole6))
  (Utilities|SetDrawerDefaults (Variables|Default|GetDresserHole7))
  (Utilities|SetDrawerDefaults (Variables|Default|GetDresserHole8))
  (Utilities|SetDrawerDefaults (Variables|Default|GetDresserHole2)))

(fn GetDrawers
  (for _array_element (Actor|GetComponentsByClass "/Script/Engine.ChildActorComponent")
    (bind _asbp_drawer_hole (Utilities|Casting|CastToBP_DrawerHole (Variables|/Script/Engine.ChildActorComponent|GetChildActor _array_element)))
    (bind _asbp_drawer_physics (Utilities|Casting|CastToBP_DrawerPhysics (Variables|/Script/Engine.ChildActorComponent|GetChildActor (Variables|/Game/HarlowsWallpaper/Interaction/Interactable_Dresser/BP_DrawerHole.BP_DrawerHole_C|GetDefaultDrawer _asbp_drawer_hole))))
    (Utilities|Array|Add (LocalVariables|GetDrawerRefs) _asbp_drawer_physics))
  (return (LocalVariables|GetDrawerRefs)))