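; Grabbable dresser drawer with axis-restricted movement that carries items placed inside it.
; Each tick it applies the drawer's change in location and rotation to "DrawerItem"-tagged actors overlapping HoldItemZone, skipping any held by a hand.
; SetHeldObjectsStatic attaches those items to the drawer actor or detaches them with physics enabled.
; Construction registers the grab zones and shows them in debug mode; MakeOnlyGrabbableByHandle destroys all but the handle zone.
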(event EventBeginPlay
  (Default|SetAxisRestrictGrab (Variables|Default|GetGrabable) (Variables|Default|GetDrawer) "/Game/UVRFProject/Framework/Hands/Model/Animations/Grabs/grab_thick_obj.grab_thick_obj" false)
  (Variables|Default|SetLastLocation (Transformation|GetWorldTransform (Variables|Default|GetDrawer))))

(event Collision|EventActorBeginOverlap
  (params (OtherActor :type Actor%20Object%20Reference)))

(event EventTick
  (params (DeltaSeconds :type Float%20%28single-precision%29))
  (bind _drawer (Variables|Default|GetDrawer))
  (bind _returnvalue (Transformation|GetWorldTransform _drawer))
  ;[1 0.3882 0.8682] Move Held objects with drawer
  (Variables|Default|SetDeltaLocation (Math|Transform|MakeTransform (- (.location _returnvalue) (.location (Variables|Default|GetLastLocation))) (Math|Rotator|Delta(Rotator) (.rotation _returnvalue) (.rotation (Variables|Default|GetLastLocation))) (.scale _returnvalue)))
  (for _array_element (Collision|GetOverlappingActors (Variables|Default|GetHoldItemZone) 0 :!class /Script/Engine.PrimitiveComponent)
    ;;[1 0.7386 0.1514] If item has a grabable and a valid hand it is being grabbed, don't move it
    (Utilities|IsValid (Actor|GetComponentbyClass _array_element "/Game/UVRFProject/Framework/Hands/Grabable.Grabable_C")
      (:Is%20Valid
        (Utilities|IsValid (Variables|/Game/UVRFProject/Framework/Hands/Grabable.Grabable_C|GetHand (Actor|GetComponentbyClass _array_element "/Game/UVRFProject/Framework/Hands/Grabable.Grabable_C"))
          (:Is%20Not%20Valid
            (bind _output_get (Variables|Default|SetHeldRootComponent (Variables|/Script/Engine.Actor|GetRootComponent _array_element))))))
      (:Is%20Not%20Valid
        _))
    (Utilities|IsValid _output_get
      (:Is%20Valid
        (if (Actor|ActorHasTag _array_element "DrawerItem")
          (Transformation|AddWorldOffset _output_get (.location (Variables|Default|GetDeltaLocation)) false false)
          (Transformation|AddWorldRotation _output_get (.rotation (Variables|Default|GetDeltaLocation)) false false)))))
  (Variables|Default|SetLastLocation (Transformation|GetWorldTransform (Variables|Default|GetDrawer))))

(fn ConstructionScript
  (bind _debugmode (Variables|Default|GetDebugMode))
  (bind _output_get (Variables|/Game/UVRFProject/Framework/Hands/Grabable.Grabable_C|SetGrabZones (Variables|Default|GetGrabable) (Utilities|Array|MakeArray (Variables|Default|GetGrabZone0) (Variables|Default|GetGrabZone1) (Variables|Default|GetGrabZone2) (Variables|Default|GetGrabZone3) (Variables|Default|GetGrabZone4) (Variables|Default|GetHandleGrabZone))))
  (for _array_element _output_get
    (Rendering|SetVisibility _array_element _debugmode false))
  (Rendering|SetVisibility (Variables|Default|GetHoldItemZone) _debugmode false))

(fn SetHeldObjectsStatic
  (params (IsStatic :type Boolean))
  (for _array_element (Collision|GetOverlappingActors (Variables|Default|GetHoldItemZone) 0 :!class /Script/Engine.PrimitiveComponent)
    (if (Actor|ActorHasTag _array_element "DrawerItem")
      (if IsStatic
        (Transformation|AttachActorToActor _array_element self "None" "KeepWorld" "KeepWorld" "KeepWorld" true)
        (else
          (Transformation|DetachFromActor _array_element "KeepWorld" "KeepWorld" "KeepWorld")
          (bind _asprimitive_component (Utilities|Casting|CastToPrimitiveComponent (Variables|/Script/Engine.Actor|GetRootComponent _array_element)))
          (Physics|SetSimulatePhysics _asprimitive_component true))))))

(fn MakeOnlyGrabbablebyHandle
  (Components|DestroyComponent (Variables|Default|GetGrabZone0))
  (Components|DestroyComponent (Variables|Default|GetGrabZone1))
  (Components|DestroyComponent (Variables|Default|GetGrabZone2))
  (Components|DestroyComponent (Variables|Default|GetGrabZone3))
  (Components|DestroyComponent (Variables|Default|GetGrabZone4)))