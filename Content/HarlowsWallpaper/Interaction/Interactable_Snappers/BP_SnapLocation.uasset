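; BP_SnapLocation is a snap point actor for the snapper interactables, marking where an overlapping object should snap to.
; On BeginPlay it falls back to its own actor transform when SnapperTransform is left at identity.
; Overlapping actors that implement Interface_Snapper receive SnappedMessage with that transform on entry and UnsnappedMessage on exit, leaving the snap behaviour to them.
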(event EventBeginPlay
  (if (== (Variables|Default|GetSnapperTransform) (Math|Transform|MakeTransform "0, 0, 0"))
    (Variables|Default|SetSnapperTransform (Transformation|GetActorTransform))))

(event Collision|EventActorBeginOverlap
  (params (OtherActor :type Actor%20Object%20Reference))
  (if (Utilities|DoesObjectImplementInterface OtherActor "/Game/HarlowsWallpaper/Interaction/Interactable_Snappers/Interface_Snapper.Interface_Snapper_C")
    (Class|InterfaceSnapper|Snapped(Message) OtherActor (Variables|Default|GetSnapperTransform))))

(event Collision|EventActorEndOverlap
  (params (OtherActor :type Actor%20Object%20Reference))
  (if (Utilities|DoesObjectImplementInterface OtherActor "/Game/HarlowsWallpaper/Interaction/Interactable_Snappers/Interface_Snapper.Interface_Snapper_C")
    (Class|InterfaceSnapper|Unsnapped(Message) OtherActor)))

(fn ConstructionScript)