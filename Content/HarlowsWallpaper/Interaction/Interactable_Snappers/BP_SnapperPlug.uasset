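; BP_SnapperPlug is a grabbable item that snaps into a given transform when held and can shatter.
; BeginPlay configures Relative, Fixed or Physics grabbing; snapping releases the hand and freezes physics.
; Hard impacts or Break swap the mesh for a destructible.
; A "slipping fingers" symptom breaks it after a timed grab, removing shards once unseen; positive values also reveal a hidden pre-made clone when its spot is unseen.
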(event GrabNotify(Grabable)
  ;[1 1 1] On Grab
  (CallFunction|SlippingActivate)
  (if (Variables|Default|GetSnapped!)
    (CallFunction|Unsnapped)))

(event OnComponentHit(ItemMeshComponent)
  (params (HitComponent :type Primitive%20Component%20Object%20Reference) (OtherActor :type Actor%20Object%20Reference) (OtherComp :type Primitive%20Component%20Object%20Reference) (NormalImpulse :type Vector :default "0, 0, 0") (Hit :type Hit%20Result%20Structure%20%28by%20ref%29))
  ;[1 1 1] Impact Destruction
  (Game|Damage|ApplyDamage self (Math|Vector|VectorLength NormalImpulse) 0 0))

(event ReleaseNotify(Grabable)
  (bind _itemmeshcomponent (Variables|Default|GetItemMeshComponent))
  ;[1 1 1] On Release
  (Physics|SetEnableGravity _itemmeshcomponent true)
  (Physics|SetSimulatePhysics _itemmeshcomponent true))

(event Custom|Break
  (bind _grabable (Variables|Default|GetGrabable))
  ;[1 1 1] Break Function
  (Variables|Default|SetDestructible true)
  (bind _returnvalue (AddComponent|AddDestructibleComponent false))
  (Class|DestructibleComponent|SetDestructibleMesh _returnvalue (Variables|Default|GetDestructibleMesh))
  (Rendering|Material|SetMaterial _returnvalue 1 (Variables|Default|GetItemMaterial))
  (Physics|SetSimulatePhysics _returnvalue true)
  (Physics|SetEnableGravity _returnvalue true)
  (Class|DestructibleComponent|ApplyRadiusDamage _returnvalue (Variables|Default|GetDestructibleDamage) (Transformation|GetActorLocation self) 3e+01 1.0 false)
  (Default|Released (Variables|Default|GetGrabable))
  (Default|ClearGrab _grabable)
  (Variables|/Game/UVRFProject/Framework/Hands/Grabable.Grabable_C|SetGrabAllowed _grabable false)
  (Components|DestroyComponent (Variables|Default|GetItemMeshComponent))
  (Variables|Default|SetDestructible false))

(event Custom|SlippingActivate
  ;[1 1 1] Slipping Fingers Symptom
  (if (!= (Variables|Default|GetSlippingFingers) 0)
    (if (> (Variables|Default|GetSlippingFingers) 0)
      (bind _returnvalue (Class|SymptomHelper|CloneActor self))
      (bind _asbp_basic_item (Utilities|Casting|CastToBP_BasicItem _returnvalue))
      (Variables|/Game/HarlowsWallpaper/Interaction/Generic_Interactable_Items/BP_BasicItem.BP_BasicItem_C|SetSlippingFingers _asbp_basic_item 0)
      (Variables|/Game/UVRFProject/Framework/Hands/Grabable.Grabable_C|SetGrabAllowed (Actor|GetComponentbyClass _asbp_basic_item "/Game/UVRFProject/Framework/Hands/Grabable.Grabable_C") false)
      (Physics|SetSimulatePhysics (Actor|GetComponentbyClass _asbp_basic_item "/Script/Engine.StaticMeshComponent") false)
      (Physics|SetEnableGravity (Actor|GetComponentbyClass _asbp_basic_item "/Script/Engine.StaticMeshComponent") false)
      (Rendering|SetVisibility (Actor|GetComponentbyClass _asbp_basic_item "/Script/Engine.StaticMeshComponent") false true)
      (Utilities|FlowControl|Delay (Math|Conversions|ToFloat(Integer) (Variables|Default|GetSlippingFingers)))
      (Variables|Default|SetSF_Location (Transformation|GetActorLocation self))
      (CallFunction|Break)
      (bind _returnvalue_2 (Class|SymptomHelper|ValidateUnseenLocation (Transformation|GetActorLocation _asbp_basic_item) self :!label _label))
      (if _returnvalue_2
        (Variables|/Game/UVRFProject/Framework/Hands/Grabable.Grabable_C|SetGrabAllowed (Actor|GetComponentbyClass _asbp_basic_item "/Game/UVRFProject/Framework/Hands/Grabable.Grabable_C") true)
        (Physics|SetSimulatePhysics (Actor|GetComponentbyClass _asbp_basic_item "/Script/Engine.StaticMeshComponent") true)
        (Physics|SetEnableGravity (Actor|GetComponentbyClass _asbp_basic_item "/Script/Engine.StaticMeshComponent") true)
        (Rendering|SetVisibility (Actor|GetComponentbyClass _asbp_basic_item "/Script/Engine.StaticMeshComponent") true true)
        (bind _returnvalue_3 (Class|SymptomHelper|ValidateUnseenLocation (Variables|Default|GetSF_Location) self :!label _label_2))
        (if _returnvalue_3
          (Actor|DestroyActor)
          (else
            (Utilities|FlowControl|Delay 1.0)
            (goto _label_2)))
        (else
          (Utilities|FlowControl|Delay 1.0)
          (goto _label)))
      (else
        (Utilities|FlowControl|Delay (Math|Float|Absolute(Float) (Math|Conversions|ToFloat(Integer) (Variables|Default|GetSlippingFingers))))
        (Variables|Default|SetSF_Location (Transformation|GetActorLocation self))
        (CallFunction|Break)
        (bind _returnvalue_4 (Class|SymptomHelper|ValidateUnseenLocation (Variables|Default|GetSF_Location) self :!label _label_3))
        (if _returnvalue_4
          (Actor|DestroyActor)
          (else
            (Utilities|FlowControl|Delay 1.0)
            (goto _label_3)))))))

(event EventSnapped
  (params (SnapTransform :type Transform))
  (bind _itemmeshcomponent (Variables|Default|GetItemMeshComponent))
  ;[1 1 1] Snapping Into Place
  (if (Default|IsGrabbed (Variables|Default|GetGrabable))
    (Default|Release (Variables|/Game/UVRFProject/Framework/Hands/Grabable.Grabable_C|GetHand (Variables|Default|GetGrabable)))
    (Transformation|SetActorTransform SnapTransform)
    (Physics|SetEnableGravity _itemmeshcomponent false)
    (Physics|SetSimulatePhysics _itemmeshcomponent false)
    (Variables|Default|SetSnapped! true)))

(event EventUnsnapped
  ;[1 1 1] Unsnapping
  (Variables|Default|SetSnapped! false))

(event Game|Damage|EventAnyDamage
  (params (Damage :type Float%20%28single-precision%29) (DamageType :type Damage%20Type%20Object%20Reference) (InstigatedBy :type Controller%20Object%20Reference) (DamageCauser :type Actor%20Object%20Reference))
  (bind _grabable (Variables|Default|GetGrabable))
  ;[1 1 1] Impact Destruction
  (if (and (Variables|Default|GetDestructible) (>= Damage (Variables|Default|GetDestructibleDamage)))
    (Development|PrintString (Utilities|String|ToString(Float) Damage))
    (bind _returnvalue (AddComponent|AddDestructibleComponent false))
    (Class|DestructibleComponent|SetDestructibleMesh _returnvalue (Variables|Default|GetDestructibleMesh))
    (Rendering|Material|SetMaterial _returnvalue 1 (Variables|Default|GetItemMaterial))
    (Physics|SetSimulatePhysics _returnvalue true)
    (Physics|SetEnableGravity _returnvalue true)
    (Class|DestructibleComponent|ApplyRadiusDamage _returnvalue Damage (Transformation|GetWorldLocation (stale OnComponentHit(ItemMeshComponent) HitComponent)) 3e+01 1.0 false)
    (Default|Released (Variables|Default|GetGrabable))
    (Default|ClearGrab _grabable)
    (Variables|/Game/UVRFProject/Framework/Hands/Grabable.Grabable_C|SetGrabAllowed _grabable false)
    (Components|DestroyComponent (Variables|Default|GetItemMeshComponent))
    (Variables|Default|SetDestructible false)))

(event EventBeginPlay
  (bind _itemmeshcomponent (Variables|Default|GetItemMeshComponent))
  (bind _grabanimation (Variables|Default|GetGrabAnimation))
  ;[1 1 1] On BeginPlay
  (switch Utilities|FlowControl|Switch|SwitchonGrabTypes (Variables|Default|GetGrabType)
    (:NewEnumerator0
      (Default|SetRelativeGrab (Variables|Default|GetGrabable) _itemmeshcomponent _grabanimation))
    (:NewEnumerator1
      (Default|SetFixedGrab (Variables|Default|GetGrabable) _itemmeshcomponent (Variables|Default|GetGrabTransformLeft) _grabanimation (Variables|Default|GetGrabTransformRight)))
    (:NewEnumerator7
      (Default|SetPhysicsGrab (Variables|Default|GetGrabable) (Variables|Default|GetItemMeshComponent) (Variables|Default|GetGrabAnimation) (Variables|Default|GetGrabDistanceMax)))))

(fn ConstructionScript
  (Components|StaticMesh|SetStaticMesh (Variables|Default|GetItemMeshComponent) (Variables|Default|GetItemMesh))
  (Rendering|Material|SetMaterial (Variables|Default|GetItemMeshComponent) 0 (Variables|Default|GetItemMaterial)))