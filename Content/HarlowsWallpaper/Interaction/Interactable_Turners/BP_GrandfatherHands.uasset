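; Grandfather clock hands puzzle where the player turns a grabbable knob, restricted to roll rotation, to set a target time.
; Tick derives minute and hour from the knob's roll, detecting wraparound to count hours and drive the hour hand pivot.
; Holding a time inside the accepted window for a short timer releases and disables the grab, sweeps both hands to midnight and plays a chime.
; Leaving the window first cancels the timer.
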(event Custom|HourHandMove
  (Components|MoveComponentTo (Variables|Default|GetHourHand) "0, 0, 0" (Math|Rotator|MakeRotator (* (+ (/ (Math|Conversions|ToFloat(Integer) (Variables|Default|GetMinute)) 6e+01) (Math|Conversions|ToFloat(Integer) (Variables|Default|GetHour))) 3.6e+02 -0.083333) 0.0 0.0) false false 1.0 true))

(event Custom|MinuteHandMove
  (Components|MoveComponentTo (Variables|Default|GetMinuteHand) "0, 0, 0" (Math|Rotator|MakeRotator (* (/ (- 6e+01 (Math|Conversions|ToFloat(Integer) (Variables|Default|GetMinute))) 5.0) 3e+01) 0.0 0.0) false false 1.0 true))

(event Custom|HandsToMidnightChime
  (bind _grabable (Variables|Default|GetGrabable))
  (Utilities|FlowControl|DoOnce false
    (:Completed
      (Default|Released _grabable)
      (Variables|/Game/UVRFProject/Framework/Hands/Grabable.Grabable_C|SetGrabAllowed _grabable false)
      (CallFunction|HourHandMove)
      (CallFunction|MinuteHandMove)
      ;[1 1 1] On BeginPlay
      (Audio|SpawnSoundatLocation "/Game/HarlowsWallpaper/SoundEffects/Clock/ClockChime_Cue.ClockChime_Cue" (Transformation|GetWorldLocation (Variables|Default|GetKnob)) "0, 0, 0" 1.0 1.0 0.0 0 0 false))))

(event EventBeginPlay
  ;[1 1 1] On BeginPlay
  (Default|SetAxisRestrictGrab (Variables|Default|GetGrabable) (Variables|Default|GetGrabberMesh) "/Game/UVRFProject/Framework/Hands/Model/Animations/Grabs/grab_brush.grab_brush" (Variables|Default|GetUseFixedGrab) (Variables|Default|GetGrabTransformLeft) (Variables|Default|GetGrabTransformRight))
  (Default|SetRestrictedAxes (Variables|Default|GetGrabable) true true true true true true false false true true true true))

(event EventTick
  (params (DeltaSeconds :type Float%20%28single-precision%29))
  (bind _hourpos (Variables|Default|GetHourPos))
  (Utilities|FlowControl|Sequence
    (:then_0
      ;[1 1 1] If time is correct, have hands return to midnight, and have sound play
      (if (Variables|Default|GetTimeCorrect)
        (Utilities|FlowControl|DoOnce false :!label _label
          (:Completed
            (bind _returnvalue (Utilities|Time|SetTimerbyEvent (delegate Custom|HandsToMidnightChime) 2.0))
            (goto _label_2 Reset)))
        (else
          (Utilities|FlowControl|DoOnce false :!label _label_2
            (:Completed
              (Utilities|Time|ClearandInvalidateTimerbyHandle _returnvalue)
              (goto _label Reset))))))
    (:then_1
      ;[1 1 1] Find Current Rotation of Knob
      (Variables|Default|SetCurrentRotation (Class|KismetMathLibrary|ClampAxis (.Roll (Math|Rotator|BreakRotator (Variables|/Script/Engine.SceneComponent|GetRelativeRotation (Variables|Default|GetGrabberMesh))))))
      ;[1 1 1] Find if Minute hand has passed 60 minutes
      (if (>= (- (Variables|Default|GetPreviousRotation) (Variables|Default|GetCurrentRotation)) 2.7e+02)
        (Math|Integer|IncrementInt _hourpos
          (:%20%20
            _))
        (elif (<= (- (Variables|Default|GetPreviousRotation) (Variables|Default|GetCurrentRotation)) -2.7e+02)
          (Math|Integer|DecrementInt _hourpos
            (:%20%20
              _))))
      ;[1 1 1] Set Hour hand Rotation
      (Variables|Default|SetPreviousRotation (Variables|Default|GetCurrentRotation))
      (Transformation|SetRelativeRotation (Variables|Default|GetHourCenter) (Math|Rotator|MakeRotator (+ (/ (Variables|Default|GetCurrentRotation) 12.0) (* (Variables|Default|GetHourPos) 3e+01)) 0.0 0.0) false false)
      ;[1 1 1] Set Hour and Minute Values
      (bind _output_get (Variables|Default|SetMinute (Math|Float|Floor (/ (Variables|Default|GetCurrentRotation) 6.0))))
      (bind _output_get_2 (Variables|Default|SetHour (Math|Float|Floor (/ (Class|KismetMathLibrary|ClampAxis (.Roll (Math|Rotator|BreakRotator (Variables|/Script/Engine.SceneComponent|GetRelativeRotation (Variables|Default|GetHourCenter))))) 3e+01))))
      (Variables|Default|SetTimeCorrect (and (and (<= _output_get 50) (>= _output_get 40)) (and (<= _output_get_2 2) (>= _output_get_2 1)))))))

(fn ConstructionScript)