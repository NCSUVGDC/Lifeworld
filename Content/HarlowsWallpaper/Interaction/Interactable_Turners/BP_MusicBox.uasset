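; BP_MusicBox is a music box interactable with a knob that is grabbed and turned to wind it, opening the lid.
; BeginPlay configures the Grabable on GrabberMesh, restricting all movement except roll.
; Tick accumulates knob rotation, counting full turns from jumps in the clamped angle.
; Once the total reaches RequiredRotation, Wound latches and the lid interpolates open.
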(event EventBeginPlay
  ;[1 1 1] On BeginPlay
  (Default|SetAxisRestrictGrab (Variables|Default|GetGrabable) (Variables|Default|GetGrabberMesh) "/Game/UVRFProject/Framework/Hands/Model/Animations/Grabs/grab_brush.grab_brush" (Variables|Default|GetUseFixedGrab) (Variables|Default|GetGrabTransformLeft) (Variables|Default|GetGrabTransformRight))
  (Default|SetRestrictedAxes (Variables|Default|GetGrabable) true true true true true true false false true true true true))

(event EventTick
  (params (DeltaSeconds :type Float%20%28single-precision%29))
  (bind _fullturns (Variables|Default|GetFullTurns))
  (if (Variables|Default|GetWound)
    ;[1 1 1] Triggered Once Wound
    (Transformation|SetRelativeRotation (Variables|Default|GetLid) (Math|Interpolation|RInterpTo (Variables|/Script/Engine.SceneComponent|GetRelativeRotation (Variables|Default|GetLid)) "0.000000, 0,-90.000000" DeltaSeconds 1.75) false false)
    (else
      ;[1 1 1] Find Current Rotation of Knob
      (Variables|Default|SetCurrentRotation (Class|KismetMathLibrary|ClampAxis (.Roll (Math|Rotator|BreakRotator (Variables|/Script/Engine.SceneComponent|GetRelativeRotation (Variables|Default|GetGrabberMesh))))))
      ;[1 1 1] Find if knob has passed 360 degrees
      (if (>= (- (Variables|Default|GetPreviousRotation) (Variables|Default|GetCurrentRotation)) 2.7e+02)
        (Math|Integer|IncrementInt _fullturns
          (:%20%20
            _))
        (elif (<= (- (Variables|Default|GetPreviousRotation) (Variables|Default|GetCurrentRotation)) -2.7e+02)
          (Math|Integer|DecrementInt _fullturns
            (:%20%20
              _))))
      (Variables|Default|SetPreviousRotation (Variables|Default|GetCurrentRotation))
      ;[1 1 1] Set total rotation value
      (bind _output_get (Variables|Default|SetKnobRotation (+ (Variables|Default|GetCurrentRotation) (Math|Conversions|ToFloat(Integer) (* (Variables|Default|GetFullTurns) 360)))))
      ;[1 1 1] Check if box has been wound
      (if (>= _output_get (Variables|Default|GetRequiredRotation))
        (Variables|Default|SetWound true)))))

(fn ConstructionScript)