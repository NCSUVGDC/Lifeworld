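; Grabbable, breakable cup that holds, pours and catches water.
; Tick caps water by a logarithmic tilt curve, spawning BP_WaterSpurt at the lowest of eight points; overlapping spurts from other actors refill it.
; Hard impacts or Break swap the mesh for a destructible and spill water.
; The SlippingFingers symptom breaks it after a post-grab delay, removes shards when unseen and, if positive, reveals a pre-made clone at the original spot.
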(event GrabNotify(Grabable)
  ;[1 1 1] On Grab
  (CallFunction|SlippingActivate))

(event OnComponentHit(ItemMeshComponent)
  (params (HitComponent :type Primitive%20Component%20Object%20Reference) (OtherActor :type Actor%20Object%20Reference) (OtherComp :type Primitive%20Component%20Object%20Reference) (NormalImpulse :type Vector :default "0, 0, 0") (Hit :type Hit%20Result%20Structure%20%28by%20ref%29))
  ;[1 1 1] Impact Destruction
  (Game|Damage|ApplyDamage self (Math|Vector|VectorLength NormalImpulse) 0 0))

(event OnComponentBeginOverlap(WaterLevel)
  (params (OverlappedComponent :type Primitive%20Component%20Object%20Reference) (OtherActor :type Actor%20Object%20Reference) (OtherComp :type Primitive%20Component%20Object%20Reference) (OtherBodyIndex :type Integer) (bFromSweep :type Boolean) (SweepResult :type Hit%20Result%20Structure%20%28by%20ref%29))
  ;[1 1 1] Water Filling
  (bind _asbp_water_spurt (Utilities|Casting|CastToBP_WaterSpurt OtherActor))
  (if (!= (Variables|/Game/HarlowsWallpaper/Interaction/Interactable_Water_Holder/BP_WaterSpurt.BP_WaterSpurt_C|GetOrigin _asbp_water_spurt) self)
    (CallFunction|WaterChanged (Variables|/Game/HarlowsWallpaper/Interaction/Interactable_Water_Holder/BP_WaterSpurt.BP_WaterSpurt_C|GetWaterAmt _asbp_water_spurt))
    (if (not (Game|IsActorBeingDestroyed OtherActor))
      (Actor|DestroyActor _asbp_water_spurt))))

(event Custom|Break
  (bind _grabable (Variables|Default|GetGrabable))
  ;[1 1 1] Break Function
  (Variables|Default|SetDestructible true)
  (bind _returnvalue (AddComponent|AddDestructibleComponent false))
  (Class|DestructibleComponent|SetDestructibleMesh _returnvalue (Variables|Default|GetDestructibleMesh))
  (Rendering|Material|SetMaterial _returnvalue 1 (Variables|Default|GetItemMaterial))
  (Physics|SetSimulatePhysics _returnvalue true)
  (Physics|SetEnableGravity _returnvalue true)
  (Class|DestructibleComponent|ApplyRadiusDamage _returnvalue (Variables|Default|GetDestructibleDamage) (Transformation|GetActorLocation self) 3e+01 1.0 false)
  (Default|Released (Variables|Default|GetGrabable))
  (Default|ClearGrab _grabable)
  (Variables|/Game/UVRFProject/Framework/Hands/Grabable.Grabable_C|SetGrabAllowed _grabable false)
  (for _array_element (Components|GetChildrenComponents (Variables|Default|GetItemMeshComponent) false)
    (if (> (Variables|Default|GetWater) 0)
      (Game|SpawnActorfromClass "/Game/HarlowsWallpaper/Interaction/Interactable_Water_Holder/BP_WaterSpurt.BP_WaterSpurt_C" (Math|Transform|MakeTransform (Transformation|GetWorldLocation _array_element) "0, 0, 0" "0.050000,0.050000,0.050000") "Undefined" 0 1 self 0))
    (Components|DestroyComponent _array_element))
  (Components|DestroyComponent (Variables|Default|GetItemMeshComponent))
  (Variables|Default|SetDestructible false)
  (Variables|Default|SetWater 0))

(event Custom|SlippingActivate
  ;[1 1 1] Slipping Fingers Symptom
  (if (!= (Variables|Default|GetSlippingFingers) 0)
    (if (> (Variables|Default|GetSlippingFingers) 0)
      (bind _returnvalue (Class|SymptomHelper|CloneActor self))
      (bind _asbp_basic_item (Utilities|Casting|CastToBP_BasicItem _returnvalue))
      (Variables|/Game/HarlowsWallpaper/Interaction/Generic_Interactable_Items/BP_BasicItem.BP_BasicItem_C|SetSlippingFingers _asbp_basic_item 0)
      (Variables|/Game/UVRFProject/Framework/Hands/Grabable.Grabable_C|SetGrabAllowed (Actor|GetComponentbyClass _asbp_basic_item "/Game/UVRFProject/Framework/Hands/Grabable.Grabable_C") false)
      (Physics|SetSimulatePhysics (Actor|GetComponentbyClass _asbp_basic_item "/Script/Engine.StaticMeshComponent") false)
      (Physics|SetEnableGravity (Actor|GetComponentbyClass _asbp_basic_item "/Script/Engine.StaticMeshComponent") false)
      (Rendering|SetVisibility (Actor|GetComponentbyClass _asbp_basic_item "/Script/Engine.StaticMeshComponent") false true)
      (Utilities|FlowControl|Delay (Math|Conversions|ToFloat(Integer) (Variables|Default|GetSlippingFingers)))
      (Variables|Default|SetSF_Location (Transformation|GetActorLocation self))
      (CallFunction|Break)
      (bind _returnvalue_2 (Class|SymptomHelper|ValidateUnseenLocation (Transformation|GetActorLocation _asbp_basic_item) self :!label _label))
      (if _returnvalue_2
        (Variables|/Game/UVRFProject/Framework/Hands/Grabable.Grabable_C|SetGrabAllowed (Actor|GetComponentbyClass _asbp_basic_item "/Game/UVRFProject/Framework/Hands/Grabable.Grabable_C") true)
        (Physics|SetSimulatePhysics (Actor|GetComponentbyClass _asbp_basic_item "/Script/Engine.StaticMeshComponent") true)
        (Physics|SetEnableGravity (Actor|GetComponentbyClass _asbp_basic_item "/Script/Engine.StaticMeshComponent") true)
        (Rendering|SetVisibility (Actor|GetComponentbyClass _asbp_basic_item "/Script/Engine.StaticMeshComponent") true true)
        (bind _returnvalue_3 (Class|SymptomHelper|ValidateUnseenLocation (Variables|Default|GetSF_Location) self :!label _label_2))
        (if _returnvalue_3
          (Actor|DestroyActor)
          (else
            (Utilities|FlowControl|Delay 1.0)
            (goto _label_2)))
        (else
          (Utilities|FlowControl|Delay 1.0)
          (goto _label)))
      (else
        (Utilities|FlowControl|Delay (Math|Float|Absolute(Float) (Math|Conversions|ToFloat(Integer) (Variables|Default|GetSlippingFingers))))
        (Variables|Default|SetSF_Location (Transformation|GetActorLocation self))
        (CallFunction|Break)
        (bind _returnvalue_4 (Class|SymptomHelper|ValidateUnseenLocation (Variables|Default|GetSF_Location) self :!label _label_3))
        (if _returnvalue_4
          (Actor|DestroyActor)
          (else
            (Utilities|FlowControl|Delay 1.0)
            (goto _label_3)))))))

(event Custom|WaterChanged
  (params (Amount :type Integer))
  ;[1 1 1] Water Filling
  (if (>= (+ Amount (Variables|Default|GetWater)) 100)
    (Variables|Default|SetWater 100)
    (else
      (Variables|Default|SetWater (Math|Integer|Clamp(Integer) (+ Amount (Variables|Default|GetWater)) 0 100))))
  (Transformation|SetRelativeScale3D (Variables|Default|GetWaterLevel) (Math|Vector|MakeVector 3.75 3.75 (* (Variables|Default|GetWater) 0.02))))

(event EventTick
  (params (DeltaSeconds :type Float%20%28single-precision%29))
  (bind _returnvalue (Transformation|GetActorRotation))
  (bind (_roll _pitch) (Math|Rotator|BreakRotator _returnvalue))
  ;[1 1 1] Water Pouring (Tick)
  (if (> (Math|Float|Absolute(Float) _roll) (Math|Float|Absolute(Float) _pitch))
    (Variables|Default|SetWaterAngle _roll)
    (else
      (Variables|Default|SetWaterAngle _pitch)))
  (Variables|Default|SetOldWater (Variables|Default|GetWater))
  (if (Math|Float|InRange(Float) (Variables|Default|GetWaterAngle) -9e+01 9e+01)
    (if (< (Math|Float|Round (|((100/(loge(91)))*(loge((91-x)))) (Math|Float|Absolute(Float) (Variables|Default|GetWaterAngle)))) (Variables|Default|GetWater))
      (Variables|Default|SetWater (Math|Float|Round (|((100/(loge(91)))*(loge((91-x)))) (Math|Float|Absolute(Float) (Variables|Default|GetWaterAngle)))))
      (Transformation|SetRelativeScale3D (Variables|Default|GetWaterLevel) (Math|Vector|MakeVector 3.75 3.75 (* (Variables|Default|GetWater) 0.02)))
      (for _array_element (Variables|Default|GetPoints) :!label _label
        (if (< (.Z (Math|Vector|BreakVector (Transformation|GetWorldLocation _array_element))) (Variables|Default|GetPointHeight))
          (Variables|Default|SetPoint _array_element)
          (Variables|Default|SetPointHeight (.Z (Math|Vector|BreakVector (Transformation|GetWorldLocation _array_element))))))
      (Variables|Default|SetPointHeight 1e+04)
      (Game|SpawnActorfromClass "/Game/HarlowsWallpaper/Interaction/Interactable_Water_Holder/BP_WaterSpurt.BP_WaterSpurt_C" (Math|Transform|MakeTransform (Transformation|GetWorldLocation (Variables|Default|GetPoint)) "0, 0, 0" "0.050000,0.050000,0.050000") "Undefined" 0 (- (Variables|Default|GetOldWater) (Variables|Default|GetWater)) self 0))
    (elif (> (Variables|Default|GetWater) 0)
      (CallFunction|WaterChanged -100)
      (goto _label))))

(event Game|Damage|EventAnyDamage
  (params (Damage :type Float%20%28single-precision%29) (DamageType :type Damage%20Type%20Object%20Reference) (InstigatedBy :type Controller%20Object%20Reference) (DamageCauser :type Actor%20Object%20Reference))
  (bind _grabable (Variables|Default|GetGrabable))
  ;[1 1 1] Impact Destruction
  (if (and (Variables|Default|GetDestructible) (>= Damage (Variables|Default|GetDestructibleDamage)))
    (Development|PrintString (Utilities|String|ToString(Float) Damage))
    (bind _returnvalue (AddComponent|AddDestructibleComponent false))
    (Class|DestructibleComponent|SetDestructibleMesh _returnvalue (Variables|Default|GetDestructibleMesh))
    (Rendering|Material|SetMaterial _returnvalue 1 (Variables|Default|GetItemMaterial))
    (Physics|SetSimulatePhysics _returnvalue true)
    (Physics|SetEnableGravity _returnvalue true)
    (Class|DestructibleComponent|ApplyRadiusDamage _returnvalue Damage (Transformation|GetWorldLocation (stale OnComponentHit(ItemMeshComponent) HitComponent)) 3e+01 1.0 false)
    (Default|Released (Variables|Default|GetGrabable))
    (Default|ClearGrab _grabable)
    (Variables|/Game/UVRFProject/Framework/Hands/Grabable.Grabable_C|SetGrabAllowed _grabable false)
    (for _array_element (Components|GetChildrenComponents (Variables|Default|GetItemMeshComponent) false)
      (if (> (Variables|Default|GetWater) 0)
        (Game|SpawnActorfromClass "/Game/HarlowsWallpaper/Interaction/Interactable_Water_Holder/BP_WaterSpurt.BP_WaterSpurt_C" (Math|Transform|MakeTransform (Transformation|GetWorldLocation _array_element) "0, 0, 0" "0.050000,0.050000,0.050000") "Undefined" 0 1 self 0))
      (Components|DestroyComponent _array_element))
    (Components|DestroyComponent (Variables|Default|GetItemMeshComponent))
    (Variables|Default|SetDestructible false)
    (Variables|Default|SetWater 0)))

(event EventBeginPlay
  (bind _itemmeshcomponent (Variables|Default|GetItemMeshComponent))
  (bind _points (Variables|Default|GetPoints))
  (bind _grabanimation (Variables|Default|GetGrabAnimation))
  (bind _points_2 (Variables|Default|GetPoints))
  ;[1 1 1] On BeginPlay
  (switch Utilities|FlowControl|Switch|SwitchonGrabTypes (Variables|Default|GetGrabType)
    (:NewEnumerator0
      (Default|SetRelativeGrab (Variables|Default|GetGrabable) _itemmeshcomponent _grabanimation))
    (:NewEnumerator1
      (Default|SetFixedGrab (Variables|Default|GetGrabable) _itemmeshcomponent (Variables|Default|GetGrabTransformLeft) _grabanimation (Variables|Default|GetGrabTransformRight)))
    (:NewEnumerator7
      (Default|SetPhysicsGrab (Variables|Default|GetGrabable) (Variables|Default|GetItemMeshComponent) (Variables|Default|GetGrabAnimation) (Variables|Default|GetGrabDistanceMax))))
  (Transformation|SetRelativeScale3D (Variables|Default|GetWaterLevel) (Math|Vector|MakeVector 3.75 3.75 (* (Variables|Default|GetWater) 0.02)))
  (Utilities|Array|Add _points_2 (Variables|Default|GetPoint1))
  (Utilities|Array|Add _points_2 (Variables|Default|GetPoint2))
  (Utilities|Array|Add _points_2 (Variables|Default|GetPoint3))
  (Utilities|Array|Add _points_2 (Variables|Default|GetPoint4))
  (Utilities|Array|Add _points (Variables|Default|GetPoint5))
  (Utilities|Array|Add _points (Variables|Default|GetPoint6))
  (Utilities|Array|Add _points (Variables|Default|GetPoint7))
  (Utilities|Array|Add _points (Variables|Default|GetPoint8)))

(fn ConstructionScript
  (Components|StaticMesh|SetStaticMesh (Variables|Default|GetItemMeshComponent) (Variables|Default|GetItemMesh))
  (Rendering|Material|SetMaterial (Variables|Default|GetItemMeshComponent) 0 (Variables|Default|GetItemMaterial)))