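; Waterable plant interactable that triggers a linked Bed to rotate down once it has received enough water.
; BP_WaterSpurt actors overlapping the Soil add their water amount and are destroyed, except spurts originating from the plant itself.
; WaterChanged accumulates the level; on reaching WaterNeeded it fixes Water at full, swaps the soil material and calls RotateDown unless the Bed is already activated or rotating.
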(event OnComponentBeginOverlap(Soil)
  (params (OverlappedComponent :type Primitive%20Component%20Object%20Reference) (OtherActor :type Actor%20Object%20Reference) (OtherComp :type Primitive%20Component%20Object%20Reference) (OtherBodyIndex :type Integer) (bFromSweep :type Boolean) (SweepResult :type Hit%20Result%20Structure%20%28by%20ref%29))
  ;[1 1 1] When Plant is Watered
  (bind _asbp_water_spurt (Utilities|Casting|CastToBP_WaterSpurt OtherActor))
  (if (!= (Variables|/Game/HarlowsWallpaper/Interaction/Interactable_Water_Holder/BP_WaterSpurt.BP_WaterSpurt_C|GetOrigin _asbp_water_spurt) self)
    (CallFunction|WaterChanged (Variables|/Game/HarlowsWallpaper/Interaction/Interactable_Water_Holder/BP_WaterSpurt.BP_WaterSpurt_C|GetWaterAmt _asbp_water_spurt))
    (if (not (Game|IsActorBeingDestroyed OtherActor))
      (Actor|DestroyActor _asbp_water_spurt))))

(event Custom|WaterChanged
  (params (Amount :type Float%20%28single-precision%29))
  (bind _bed (Variables|Default|GetBed))
  ;[1 1 1] Change Water Level of Plant
  (if (>= (+ Amount (Variables|Default|GetWater)) (Variables|Default|GetWaterNeeded))
    (Variables|Default|SetWater 1e+02)
    (Rendering|Material|SetMaterial (Variables|Default|GetSoil) 0 "/Game/HarlowsWallpaper/Materials/Wallpaper/HeadLocked_Mat.HeadLocked_Mat")
    (if (and (not (Variables|/Game/HarlowsWallpaper/Interaction/Bed/Bed.Bed_C|GetActivated _bed)) (not (Variables|/Game/HarlowsWallpaper/Interaction/Bed/Bed.Bed_C|GetRotateDown? _bed)))
      (Default|RotateDown (Variables|Default|GetBed)))
    (else
      (Variables|Default|SetWater (+ Amount (Variables|Default|GetWater))))))

(fn ConstructionScript)