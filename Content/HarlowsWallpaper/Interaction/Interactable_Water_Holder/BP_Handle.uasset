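; Grabbable water-holder handle that turns around yaw within a limited range to control a Spurter.
; Grabable locks all translation, roll and pitch; each Tick clamps yaw between StartYaw and MaxRotation beyond it, blocking further rotation at either limit and snapping overshoots past 100 degrees to the opposite end.
; Yaw maps inversely to Spurter Frequency, activating it once turned far enough; only snapping to the minimum deactivates it.
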(event Custom|RestrictMax
  (bind _handle (Variables|Default|GetHandle))
  (bind _relativerotation (Variables|/Script/Engine.SceneComponent|GetRelativeRotation _handle))
  ;[1 1 1] Restrict Handle Turning Maximum Value
  (if (>= (Class|KismetMathLibrary|ClampAxis (.Yaw (Math|Rotator|BreakRotator _relativerotation))) (+ (Variables|Default|GetStartYaw) (Variables|Default|GetMaxRotation)))
    (if (>= (Class|KismetMathLibrary|ClampAxis (.Yaw (Math|Rotator|BreakRotator _relativerotation))) (+ (Variables|Default|GetStartYaw) (Variables|Default|GetMaxRotation) 1e+02))
      (CallFunction|OverwriteMin)
      (else
        (Default|SetRestrictedAxes (Variables|Default|GetGrabable) true true true true true true true true true true true false)
        (Transformation|SetRelativeRotation (Variables|Default|GetHandle) (Math|Rotator|MakeRotator 0.0 0.0 (+ (Variables|Default|GetStartYaw) (Variables|Default|GetMaxRotation) -1.0)) false false)))
    (else
      (Default|SetRestrictedAxes (Variables|Default|GetGrabable) true true true true true true true true true true false false))))

(event Custom|RestrictMin
  (bind _handle (Variables|Default|GetHandle))
  (bind _relativerotation (Variables|/Script/Engine.SceneComponent|GetRelativeRotation _handle))
  ;[1 1 1] Restrict Handle Turning Minimum Value
  (if (<= (Class|KismetMathLibrary|ClampAxis (.Yaw (Math|Rotator|BreakRotator _relativerotation))) (Variables|Default|GetStartYaw))
    (if (<= (Class|KismetMathLibrary|ClampAxis (.Yaw (Math|Rotator|BreakRotator _relativerotation))) (- (Variables|Default|GetStartYaw) 1e+02))
      (CallFunction|OverwriteMax)
      (else
        (Default|SetRestrictedAxes (Variables|Default|GetGrabable) true true true true true true true true true true false true)
        (Variables|/Game/HarlowsWallpaper/Interaction/Interactable_Water_Holder/BP_Spurter.BP_Spurter_C|SetActivated (Variables|Default|GetSpurter) false)
        (Transformation|SetRelativeRotation (Variables|Default|GetHandle) (Math|Rotator|MakeRotator 0.0 0.0 (+ (Variables|Default|GetStartYaw) 1.0)) false false)))
    (else
      (CallFunction|RestrictMax))))

(event Custom|OverwriteMax
  ;[1 1 1] Restrict Handle Turning Maximum Value
  (Transformation|SetRelativeRotation (Variables|Default|GetHandle) (Math|Rotator|MakeRotator 0.0 0.0 (+ (Variables|Default|GetStartYaw) (Variables|Default|GetMaxRotation) -1.0)) false false))

(event Custom|OverwriteMin
  ;[1 1 1] Restrict Handle Turning Minimum Value
  (Variables|/Game/HarlowsWallpaper/Interaction/Interactable_Water_Holder/BP_Spurter.BP_Spurter_C|SetActivated (Variables|Default|GetSpurter) false)
  (Transformation|SetRelativeRotation (Variables|Default|GetHandle) (Math|Rotator|MakeRotator 0.0 0.0 (+ (Variables|Default|GetStartYaw) 1.0)) false false))

(event EventBeginPlay
  ;[1 1 1] On BeginPlay
  (Default|SetAxisRestrictGrab (Variables|Default|GetGrabable) (Variables|Default|GetHandle) "/Game/UVRFProject/Framework/Hands/Model/Animations/Grabs/grab_brush.grab_brush" (Variables|Default|GetUseFixedGrab) (Variables|Default|GetGrabTransformLeft) (Variables|Default|GetGrabTransformRight))
  (Default|SetRestrictedAxes (Variables|Default|GetGrabable) true true true true true true true true true true false false)
  (Variables|Default|SetStartYaw (Class|KismetMathLibrary|ClampAxis (.Yaw (Math|Rotator|BreakRotator (Variables|/Script/Engine.SceneComponent|GetRelativeRotation (Variables|Default|GetHandle)))))))

(event EventTick
  (params (DeltaSeconds :type Float%20%28single-precision%29))
  (bind _startyaw (Variables|Default|GetStartYaw))
  ;[1 1 1] Restrict Handle Angle and Set Spurter Frequency (On Tick)
  (CallFunction|RestrictMin)
  (bind _output_get (Variables|/Game/HarlowsWallpaper/Interaction/Interactable_Water_Holder/BP_Spurter.BP_Spurter_C|SetFrequency (Variables|Default|GetSpurter) (Math|Float|MapRangeClamped (Class|KismetMathLibrary|ClampAxis (.Yaw (Math|Rotator|BreakRotator (Variables|/Script/Engine.SceneComponent|GetRelativeRotation (Variables|Default|GetHandle))))) _startyaw (+ _startyaw (Variables|Default|GetMaxRotation)) (* (Variables|Default|GetMaxFrequency) 1e+01) (Variables|Default|GetMaxFrequency))))
  (if (< _output_get (* (Variables|Default|GetMaxFrequency) 9.0))
    (Variables|/Game/HarlowsWallpaper/Interaction/Interactable_Water_Holder/BP_Spurter.BP_Spurter_C|SetActivated (Variables|Default|GetSpurter) true)
    (elif (> _output_get (Variables|Default|GetMaxFrequency))
      _)))

(fn ConstructionScript)