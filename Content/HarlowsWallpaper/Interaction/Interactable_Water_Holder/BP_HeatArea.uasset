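; BP_HeatArea is a heat zone that switches a Box's collision according to its HeatValue.
; Tick compares HeatValue to ActiveThreshold, setting query-only collision at or above it and no collision below.
; Two cross-resetting DoOnce nodes limit each switch to one call per threshold crossing.
; Debug prints read "Heat Disabled" when collision turns on and "Heat Enabled" when it turns off.
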(event EventBeginPlay)

(event Collision|EventActorBeginOverlap
  (params (OtherActor :type Actor%20Object%20Reference)))

(event EventTick
  (params (DeltaSeconds :type Float%20%28single-precision%29))
  (if (>= (Variables|Default|GetHeatValue) (Variables|Default|GetActive%20Threshold))
    (Utilities|FlowControl|Sequence
      (:then_0
        (Utilities|FlowControl|DoOnce false :!label _label
          (:Completed
            (Collision|SetCollisionEnabled (Variables|Default|GetBox) "QueryOnly")
            (Development|PrintString "Heat Disabled"))))
      (:then_1
        (goto _label_2 Reset)))
    (else
      (Utilities|FlowControl|Sequence
        (:then_0
          (Utilities|FlowControl|DoOnce false :!label _label_2
            (:Completed
              (Collision|SetCollisionEnabled (Variables|Default|GetBox) "NoCollision")
              (Development|PrintString "Heat Enabled"))))
        (:then_1
          (goto _label Reset))))))

(fn ConstructionScript)