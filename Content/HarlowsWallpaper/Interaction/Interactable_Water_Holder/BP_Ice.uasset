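; BP_Ice is a grabbable ice block that drips water and melts away while overlapping a BP_HeatArea.
; BeginPlay configures relative, fixed or physics grabbing and records starting volume and scale.
; Tick uses DoOnce gates to swap one looping timer between passive dripping and melting, both spawning BP_WaterSpurt actors.
; Melting reduces volume, shrinking the cube by the cube root of the remaining fraction until destroyed; passive drips leave volume untouched.
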(event EventTick
  (params (DeltaSeconds :type Float%20%28single-precision%29))
  ;[1 1 1] Check if the ice is melting
  (Physics|SetEnableGravity (Variables|Default|GetCube) true)
  (if (Variables|Ice|GetIsMelting)
    (Utilities|FlowControl|Sequence
      (:then_0
        (Utilities|FlowControl|DoOnce false :!label _label
          (:Completed
            (Utilities|Time|ClearandInvalidateTimerbyHandle (Variables|Ice|GetCurrentTimer))
            (bind _returnvalue (Utilities|Time|SetTimerbyFunctionName 0 "Melting" (/ 1.0 (Variables|Ice|GetMeltingDripRate)) true))
            (Variables|Ice|SetCurrentTimer _returnvalue))))
      (:then_1
        (goto _label_2 Reset)))
    (else
      (Utilities|FlowControl|Sequence
        (:then_0
          (Utilities|FlowControl|DoOnce false :!label _label_2
            (:Completed
              (Utilities|Time|ClearandInvalidateTimerbyHandle (Variables|Ice|GetCurrentTimer))
              (bind _returnvalue_2 (Utilities|Time|SetTimerbyFunctionName 0 "PassiveDripping" (/ 1.0 (Variables|Ice|GetPassiveDripRate)) true))
              (Variables|Ice|SetCurrentTimer _returnvalue_2))))
        (:then_1
          (goto _label Reset))))))

(event Collision|EventActorBeginOverlap
  (params (OtherActor :type Actor%20Object%20Reference))
  ;[1 1 1] Switch the melting state based on overlapping with heated area
  (Utilities|Casting|CastToBP_HeatArea OtherActor)
  (Variables|Ice|SetIsMelting true))

(event Collision|EventActorEndOverlap
  (params (OtherActor :type Actor%20Object%20Reference))
  ;[1 1 1] Switch the melting state based on overlapping with heated area
  (Utilities|Casting|CastToBP_HeatArea OtherActor)
  (Variables|Ice|SetIsMelting false))

(event EventBeginPlay
  (bind _cube (Variables|Default|GetCube))
  (bind _grabanimation (Variables|Default|GetGrabAnimation))
  (Utilities|FlowControl|Sequence
    (:then_0
      ;[1 1 1] On BeginPlay
      (switch Utilities|FlowControl|Switch|SwitchonGrabTypes (Variables|Default|GetGrabType)
        (:NewEnumerator0
          (Default|SetRelativeGrab (Variables|Default|GetGrabable) _cube _grabanimation))
        (:NewEnumerator1
          (Default|SetFixedGrab (Variables|Default|GetGrabable) _cube (Variables|Default|GetGrabTransformLeft) _grabanimation (Variables|Default|GetGrabTransformRight)))
        (:NewEnumerator7
          (Default|SetPhysicsGrab (Variables|Default|GetGrabable) (Variables|Default|GetCube) (Variables|Default|GetGrabAnimation) (Variables|Default|GetGrabDistanceMax)))))
    (:then_1
      ;;[1 1 1] Set Water Volume in Ice
      (Variables|Ice|SetCurrentVolume (Variables|Ice|GetInitialVolume))
      (Variables|Ice|SetOriginalScale (Transformation|GetWorldScale (Variables|Default|GetCube))))))

(fn ConstructionScript)

(fn Melting
  (bind _self self)
  (bind _originalscale (Variables|Ice|GetOriginalScale))
  (Utilities|FlowControl|FlipFlop
    (:A
      (Game|SpawnActorfromClass "/Game/HarlowsWallpaper/Interaction/Interactable_Water_Holder/BP_WaterSpurt.BP_WaterSpurt_C" (Math|Transform|MakeTransform (.location (Transformation|GetWorldTransform (Variables|Default|GetCube))) "0, 0, 0" "0.020000,0.010000,0.010000") "Undefined" _self (Variables|Ice|GetMeltingDripVolume) _self 0))
    (:B
      _))
  (bind _output_get (Variables|Ice|SetCurrentVolume (- (Variables|Ice|GetCurrentVolume) (Variables|Ice|GetMeltingDripVolume))))
  (if (> _output_get 0.0)
    (Transformation|SetWorldScale3D (Variables|Default|GetCube) (Math|Vector|MakeVector (Math|Float|Power (* (/ (Variables|Ice|GetCurrentVolume) (Variables|Ice|GetInitialVolume)) (Math|Float|Power (.x _originalscale) 3.0)) (/ 1.0 3.0)) (Math|Float|Power (* (/ (Variables|Ice|GetCurrentVolume) (Variables|Ice|GetInitialVolume)) (Math|Float|Power (.y _originalscale) 3.0)) (/ 1.0 3.0)) (Math|Float|Power (* (/ (Variables|Ice|GetCurrentVolume) (Variables|Ice|GetInitialVolume)) (Math|Float|Power (.z _originalscale) 3.0)) (/ 1.0 3.0))))
    (else
      (Actor|DestroyActor))))

(fn PassiveDripping
  (bind _cube (Variables|Default|GetCube))
  (bind _returnvalue (Transformation|GetWorldTransform _cube))
  (Game|SpawnActorfromClass "/Game/HarlowsWallpaper/Interaction/Interactable_Water_Holder/BP_WaterSpurt.BP_WaterSpurt_C" (Math|Transform|MakeTransform (.location _returnvalue) (.rotation _returnvalue) "0.010000,0.010000,0.010000") "Undefined" 0 (Variables|Ice|GetPassiveDripVolume) 0 0))