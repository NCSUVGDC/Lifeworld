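; BP_IceChunk is an ice chunk that drips water by spawning BP_WaterSpurt actors at its mesh.
; Tick watches IsMelting and uses DoOnce gates to swap one looping timer between the melting and passive drip rates.
; Each melting drip subtracts from the current volume and rescales the mesh by an approximate cube root, so size follows remaining volume.
; Passive drips spawn water without reducing volume.
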(event EventTick
  (params (DeltaSeconds :type Float%20%28single-precision%29))
  (bind _passive_drip_rate (Variables|Default|GetPassive%20Drip%20Rate))
  (bind _returnvalue (/ 1.0 _passive_drip_rate))
  (if (Variables|Default|GetIs%20Melting)
    (Utilities|FlowControl|Sequence
      (:then_0
        (Utilities|FlowControl|DoOnce false :!label _label
          (:Completed
            (Utilities|Time|ClearandInvalidateTimerbyHandle (Variables|Default|GetCurrent%20Timer))
            (bind _returnvalue_2 (Utilities|Time|SetTimerbyFunctionName 0 "Melting" (/ 1.0 (Variables|Default|GetMelting%20Drip%20Rate)) true))
            (Variables|Default|SetCurrent%20Timer _returnvalue_2))))
      (:then_1
        (goto _label_2 Reset)))
    (else
      (Utilities|FlowControl|Sequence
        (:then_0
          (Utilities|FlowControl|DoOnce false :!label _label_2
            (:Completed
              (Utilities|FlowControl|Delay _returnvalue)
              (Utilities|Time|ClearandInvalidateTimerbyHandle (Variables|Default|GetCurrent%20Timer))
              (bind _returnvalue_3 (Utilities|Time|SetTimerbyFunctionName 0 "Passive Dripping" _returnvalue true))
              (Variables|Default|SetCurrent%20Timer _returnvalue_3))))
        (:then_1
          (goto _label Reset))))))

(event EventBeginPlay
  (Variables|Default|SetCurrent%20Volume (Variables|Default|GetInitial%20Volume)))

(fn ConstructionScript
  (Variables|Default|SetOriginal%20Scale (.X (Math|Vector|BreakVector "0, 0, 0"))))

(fn PassiveDripping
  (Game|SpawnActorfromClass "/Game/HarlowsWallpaper/Interaction/Interactable_Water_Holder/BP_WaterSpurt.BP_WaterSpurt_C" (Transformation|GetWorldTransform (Variables|Default|GetItemMeshComponent)) "Undefined" 0 (Variables|Default|GetPassive%20Drip%20Volume) 0 0))

(fn Melting
  (Game|SpawnActorfromClass "/Game/HarlowsWallpaper/Interaction/Interactable_Water_Holder/BP_WaterSpurt.BP_WaterSpurt_C" (Transformation|GetWorldTransform (Variables|Default|GetItemMeshComponent)) "Undefined" 0 (Variables|Default|GetMelting%20Drip%20Volume) 0 0)
  (Variables|Default|SetCurrent%20Volume (- (Variables|Default|GetCurrent%20Volume) (Variables|Default|GetMelting%20Drip%20Volume)))
  (Transformation|SetRelativeScale3D (Variables|Default|GetItemMeshComponent) (Math|Vector|MakeVector (Math|Float|Power (* (/ (Variables|Default|GetCurrent%20Volume) (Variables|Default|GetInitial%20Volume)) (Math|Float|Power (Variables|Default|GetOriginal%20Scale) 3.0)) 0.33) (Math|Float|Power (* (/ (Variables|Default|GetCurrent%20Volume) (Variables|Default|GetInitial%20Volume)) (Math|Float|Power (Variables|Default|GetOriginal%20Scale) 3.0)) 0.33) (Math|Float|Power (* (/ (Variables|Default|GetCurrent%20Volume) (Variables|Default|GetInitial%20Volume)) (Math|Float|Power (Variables|Default|GetOriginal%20Scale) 3.0)) 0.33))))