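; BP_IceSpurter is an ice dispenser that repeatedly spawns BP_Ice at its Cube component while Activated.
; Tick polls Activated, using paired DoOnce gates that re-arm each other to start a looping timer on activation and clear it on deactivation.
; DroppingRate sets spawns per second, IceSize sets uniform scale, and drip, melting and initial volume settings pass to each spawned ice.
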(event Custom|Spawn%20Ice
  (bind _ice_size (Variables|Default|GetIce%20Size))
  ;[1 1 1] Make Ice
  (Game|SpawnActorfromClass "/Game/HarlowsWallpaper/Interaction/Interactable_Water_Holder/BP_Ice.BP_Ice_C" (Math|Transform|MakeTransform (Transformation|GetWorldLocation (Variables|Default|GetCube)) "0, 0, 0" (Math|Vector|MakeVector _ice_size _ice_size _ice_size)) "Undefined" 0 (Variables|Default|GetPassive%20Drip%20Rate) (Variables|Default|GetPassive%20Drip%20Volume) (Variables|Default|GetMelting%20Drip%20Rate) (Variables|Default|GetMelting%20Drip%20Volume) (Variables|Default|GetInitial%20Volume) 0))

(event EventTick
  (params (DeltaSeconds :type Float%20%28single-precision%29))
  ;[1 1 1] Make Ice
  (if (Variables|Default|GetActivated)
    (Utilities|FlowControl|Sequence
      (:then_0
        (Utilities|FlowControl|DoOnce false :!label _label
          (:Completed
            (bind _returnvalue (Utilities|Time|SetTimerbyEvent (delegate Custom|Spawn%20Ice) (/ 1.0 (Variables|Default|GetDropping%20Rate)) true))
            (Variables|Default|SetCurrentTimer _returnvalue))))
      (:then_1
        (goto _label_2 Reset)))
    (else
      (Utilities|FlowControl|Sequence
        (:then_0
          (Utilities|FlowControl|DoOnce false :!label _label_2
            (:Completed
              (Utilities|Time|ClearandInvalidateTimerbyHandle (Variables|Default|GetCurrentTimer)))))
        (:then_1
          (goto _label Reset))))))

(fn ConstructionScript)