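; BP_Spurter is a water emitter that releases bursts of BP_WaterSpurt actors while Activated.
; Each burst spawns a Spread-driven number of small spurts at the Sphere's height, randomly offset horizontally within SpreadDist, passing WaterSize as their water amount.
; Tick drives the bursts, using the Drip flag and a Delay of Frequency as a gate between them.
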(event EventBeginPlay)

(event Collision|EventActorBeginOverlap
  (params (OtherActor :type Actor%20Object%20Reference)))

(event EventTick
  (params (DeltaSeconds :type Float%20%28single-precision%29))
  (bind _sphere (Variables|Default|GetSphere))
  (bind _returnvalue (Transformation|GetWorldLocation _sphere))
  (bind (_x _y _z) (Math|Vector|BreakVector _returnvalue))
  (if (and (Variables|Default|GetDrip?) (Variables|Default|GetActivated))
    (for _index (range 0 (Variables|Default|GetSpread))
      (Game|SpawnActorfromClass "/Game/HarlowsWallpaper/Interaction/Interactable_Water_Holder/BP_WaterSpurt.BP_WaterSpurt_C" (Math|Transform|MakeTransform (Math|Vector|MakeVector (+ (Math|Random|RandomFloatinRange (* (Variables|Default|GetSpreadDist) -1.0) (Variables|Default|GetSpreadDist)) _x) (+ _y (Math|Random|RandomFloatinRange (* (Variables|Default|GetSpreadDist) -1.0) (Variables|Default|GetSpreadDist))) _z) "0, 0, 0" "0.050000,0.050000,0.050000") "Undefined" 0 (Variables|Default|GetWaterSize) 0 0))
    (Variables|Default|SetDrip? false)
    (Utilities|FlowControl|Delay (Variables|Default|GetFrequency))
    (Variables|Default|SetDrip? true)))

(fn ConstructionScript)