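; BP_Key_Bit is a grabbable key piece that combines with a key handle to form a usable key.
; At BeginPlay it sets up physics grab and defaults an unset snap transform to its own.
; Overlapping a Snapper-interface actor tagged KeyHandle sends that actor a snap message.
; The bit then spawns the key Blueprint in its place, passes on its lock ID and destroys itself.
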(event Collision|EventActorBeginOverlap
  (params (OtherActor :type Actor%20Object%20Reference))
  ;[1 1 1] Snaps Object into Place
  (if (and (Utilities|DoesObjectImplementInterface OtherActor "/Game/HarlowsWallpaper/Interaction/Interactable_Snappers/Interface_Snapper.Interface_Snapper_C") (Actor|ActorHasTag OtherActor "KeyHandle"))
    (Class|InterfaceSnapper|Snapped(Message) OtherActor (Variables|Default|GetSnapperTransform) "KeyBit")
    ;[1 1 1] Spawn actual key and destroy object
    (bind _returnvalue (Game|SpawnActorfromClass "/Game/HarlowsWallpaper/Interaction/Interactable_keys_locks/Key_BP.Key_BP_C" (Transformation|GetActorTransform) "Undefined" 0 0))
    (Variables|/Game/HarlowsWallpaper/Interaction/Interactable_keys_locks/Key_BP.Key_BP_C|SetLock_Key_ID _returnvalue (Variables|Default|GetLock%20KeyBit%20ID))
    (Actor|DestroyActor)))

(event EventBeginPlay
  (Default|SetPhysicsGrab (Variables|Default|GetGrabable) (Variables|Default|GetKey_Loop) (Variables|Default|GetGrabAnimation) (Variables|Default|GetGrabDistanceMax))
  ;[1 1 1] Sets Snap Location
  (if (== (Variables|Default|GetSnapperTransform) (Math|Transform|MakeTransform "0, 0, 0"))
    (Variables|Default|SetSnapperTransform (Transformation|GetActorTransform))))

(fn ConstructionScript)