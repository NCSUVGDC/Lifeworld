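; BP_Key_Loop is a grabbable key loop that combines with a key shaft to form a complete key.
; At BeginPlay it configures its Grabable component with axis-restricted grab settings, a brush grab animation and left/right hand transforms.
; On release, it measures the distance to the first BP_Key_Shaft found in the level.
; If that shaft is very close, it destroys both pieces and spawns Key_BP at the loop's transform.
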(event ReleaseNotify(Grabable)
  (bind _outactors (Actor|GetAllActorsOfClass "/Game/HarlowsWallpaper/Interaction/Interactable_keys_locks/BP_Key_Shaft.BP_Key_Shaft_C"))
  (if (< (Math|Vector|VectorLength (- (Transformation|GetActorLocation (Utilities|Array|Get(acopy) _outactors)) (Transformation|GetActorLocation))) 1e+01)
    (Actor|DestroyActor (Utilities|Array|Get(acopy) _outactors))
    (Game|SpawnActorfromClass "/Game/HarlowsWallpaper/Interaction/Interactable_keys_locks/Key_BP.Key_BP_C" (Transformation|GetActorTransform) "Undefined" 0 0)
    (Actor|DestroyActor)))

(event EventBeginPlay
  (bind _grabable (Variables|Default|GetGrabable))
  (Default|SetAxisRestrictGrab _grabable (Variables|Default|GetKey_Loop) "/Game/UVRFProject/Framework/Hands/Model/Animations/Grabs/grab_brush.grab_brush" true (Variables|Default|GetGrabTransformLeft) (Variables|Default|GetGrabTransformRight))
  (Default|SetRestrictedAxes _grabable false false false false false false false false false false false false))

(fn ConstructionScript)