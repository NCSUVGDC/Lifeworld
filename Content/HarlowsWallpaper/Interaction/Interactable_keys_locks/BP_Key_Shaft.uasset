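; BP_Key_Shaft is the shaft piece of a key, a grabbable physics object that can snap into place.
; On BeginPlay its Grabable component sets up physics grabbing on the KeyShaft mesh.
; When Snapped fires while held, it clears the grab, teleports to the snap transform, disables gravity and physics, then destroys itself.
; Unconnected nodes for removing a nearby BP_Key_Loop and spawning Key_BP never run.
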(event ReleaseNotify(Grabable)
  ;[1 1 1] Destroy when snapped
)

(event EventSnapped
  (params (SnapTransform :type Transform))
  (bind _key_shaft (Variables|Default|GetKey_Shaft))
  ;[1 1 1] Snapping Into Place
  (if (Default|IsGrabbed (Variables|Default|GetGrabable))
    (Default|ClearGrab (Variables|Default|GetGrabable))
    (Transformation|SetActorTransform SnapTransform)
    (Physics|SetEnableGravity _key_shaft false)
    (Physics|SetSimulatePhysics _key_shaft false)
    (Variables|Default|SetSnapped! true)
    ;[1 1 1] destroy object
    (Actor|DestroyActor)))

(event EventBeginPlay
  (Default|SetPhysicsGrab (Variables|Default|GetGrabable) (Variables|Default|GetKey_Shaft) (Variables|Default|GetGrabAnimation) (Variables|Default|GetGrabDistanceMax)))

(fn ConstructionScript)