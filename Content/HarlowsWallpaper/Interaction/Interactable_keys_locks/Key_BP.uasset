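; Key actor for the lock-and-key interaction system, identified by a LockKeyID and picked up through a Grabable component.
; On BeginPlay it configures the Grabable with the PhKey volume, a borrowed brush grab animation and left/right hand transforms, then applies restricted axes.
; The construction script writes the ID to an EditorID text label, with a toggle to hide it in game.
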(event EventBeginPlay
  (bind _grabable (Variables|Default|GetGrabable))
  (Default|SetAxisRestrictGrab _grabable (Variables|Default|Getph_key) "/Game/UVRFProject/Framework/Hands/Model/Animations/Grabs/grab_brush.grab_brush" (Variables|Default|GetFixedGrabWhenUnrestricted) (Variables|Default|GetGrabTransformLeft) (Variables|Default|GetGrabTransformRight))
  (Default|SetRestrictedAxes _grabable false false false false false false false false false false false false))

(event EventTick
  (params (DeltaSeconds :type Float%20%28single-precision%29)))

(event Collision|EventActorBeginOverlap
  (params (OtherActor :type Actor%20Object%20Reference)))

(event Collision|EventActorEndOverlap
  (params (OtherActor :type Actor%20Object%20Reference)))

(fn ConstructionScript
  (bind _editor_id (Variables|Default|GetEditor_ID))
  (Rendering|Components|TextRender|SetText _editor_id (Utilities|Text|ToText(String) (Variables|Default|GetLock_Key_ID)))
  (Development|SetHiddeninGame _editor_id (Variables|Default|GetLabelHiddenInGame) false))