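; Keyed lock that accepts a held, aligned key and unlocks when a matching key is turned.
; Keyhole overlap snaps and attaches the key with physics off.
; A Tick-driven state machine follows insertion depth and roll, restricting the grabbable's axes per state so mismatched keys cannot turn.
; Unlock fires an event, releases the key, then either sets DoorOpen or replaces the lock with dummy body and bolt actors.
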(event OnComponentBeginOverlap(Keyhole)
  (params (OverlappedComponent :type Primitive%20Component%20Object%20Reference) (OtherActor :type Actor%20Object%20Reference) (OtherComp :type Primitive%20Component%20Object%20Reference) (OtherBodyIndex :type Integer) (bFromSweep :type Boolean) (SweepResult :type Hit%20Result%20Structure%20%28by%20ref%29))
  ;[0.3047 1 0.2011] Key is in keyhole
  (if (and (Components|ComponentHasTag OtherComp "KeyTip") (Variables|Default|GetKeyholeOpen)) ; Overlapped with key teeth hit box and is accepting keys
    (bind _askey_bp (Utilities|Casting|CastToKey_BP OtherActor))
    (Utilities|IsValid (Variables|/Game/UVRFProject/Framework/Hands/Grabable.Grabable_C|GetHand (Variables|/Game/HarlowsWallpaper/Interaction/Interactable_keys_locks/Key_BP.Key_BP_C|GetGrabable _askey_bp)) ; If it is being held. (Throwing key into hole doesn't make sense)
      (:Is%20Valid
        (Variables|Default|SetKey _askey_bp)
        ;[0.1415 0.1413 1] Check if key is aligned correctly to be in hole
        (if (Math|Rotator|Equal(Rotator) (.rotation (Class|KismetMathLibrary|ConvertTransformtoRelative (Transformation|GetActorTransform (Variables|Default|GetKey)) (Transformation|GetActorTransform self))) "0, 0, 0" (Variables|Default|GetKeyInsertRotationTolerance)) ; If key is rightside up (within tolerance)
          (CallFunction|SnapKeytoInsertPosition)
          (Variables|Default|SetLockState "NewEnumerator0")
          (Variables|Default|SetAreProperAxesRestricted false)
          (Variables|Default|SetKeyholeOpen false))))))

(event EventBeginPlay)

(event Collision|EventActorBeginOverlap
  (params (OtherActor :type Actor%20Object%20Reference)))

(event EventTick
  (params (DeltaSeconds :type Float%20%28single-precision%29))
  (if (Utilities|IsValid (Variables|Default|GetKey))
    (switch Utilities|FlowControl|Switch|SwitchonLockTurningStates (Variables|Default|GetLockState)
      (:NewEnumerator4
        (KeyStateTicks|NoKeyTick))
      (:NewEnumerator0
        (KeyStateTicks|KeyInsertedTick))
      (:NewEnumerator1
        (KeyStateTicks|KeyFullyInsertedTick))
      (:NewEnumerator2
        (KeyStateTicks|KeyBeginsRotationTick))
      (:NewEnumerator3
        (KeyStateTicks|KeyFullyRotatedTick)))))

(fn ConstructionScript
  (if (Variables|Default|GetBedroomDoor?)
    (Collision|SetCollisionResponsetoChannel (Variables|Default|Getlock_bolt_mesh) "ECC_GameTraceChannel2" "ECR_Ignore"))
  (Rendering|Components|TextRender|SetText (Variables|Default|GetEditor_ID) (Utilities|Text|ToText(String) (Variables|Default|GetLock_Key_ID))) ; Set the editor ID text
  ;[1 1 1] Start locked/unlocked
  (if (Variables|Default|GetStartLocked)
    (CallFunction|Lock)
    (else
      (CallFunction|Unlock))))

(fn Lock
  (Variables|Default|SetisLocked true)
  (Default|CallLockEvent)
  (Development|PrintString (Utilities|String|Append "Locking Lock ID: " (Variables|Default|GetLock_Key_Id))))

(fn Unlock
  (bind _scene (Variables|Default|GetScene))
  (bind _returnvalue (Transformation|GetWorldTransform _scene))
  (if (Variables|Default|GetisLocked)
    (Variables|Default|SetisLocked false)
    (Default|CallUnlockEvent)
    (CallFunction|RemoveKey)
    (Variables|Default|SetKeyholeOpen false) ; Don't allow new key
    ;[1 1 1] Spawn dummy parts
    (if (Variables|Default|GetNeedDummyParts?)
      (Game|SpawnActorfromClass "/Game/HarlowsWallpaper/Interaction/Interactable_keys_locks/BP_DummyLockBody.BP_DummyLockBody_C" (Math|Transform|ComposeTransforms (Variables|Default|GetDummyLockTransform) _returnvalue) "AlwaysSpawn" 0 0)
      (Game|SpawnActorfromClass "/Game/HarlowsWallpaper/Interaction/Interactable_keys_locks/BP__DummyLockBolt.BP__DummyLockBolt_C" (Math|Transform|ComposeTransforms (Variables|Default|GetDummyBoltTransform) _returnvalue) "AlwaysSpawn" 0 0)
      (Actor|DestroyActor)
      (else
        (Variables|Default|SetDoorOpen? true)))))

(fn SnapKeytoInsertPosition
  (bind _key (Variables|Default|GetKey))
  (bind _key_2 (Variables|Default|GetKey))
  (bind _grabable (Variables|/Game/HarlowsWallpaper/Interaction/Interactable_keys_locks/Key_BP.Key_BP_C|GetGrabable _key))
  (bind _ph_key (Variables|/Game/HarlowsWallpaper/Interaction/Interactable_keys_locks/Key_BP.Key_BP_C|Getph_key _key))
  (Development|PrintString "Snapping")
  (Transformation|AttachActorToActor _key_2 self "None" "KeepWorld" "KeepWorld" "KeepWorld" false)
  (Development|PrintString (Utilities|String|Append "Key Parent" (Utilities|GetDisplayName (Transformation|GetAttachParent (Variables|/Game/HarlowsWallpaper/Interaction/Interactable_keys_locks/Key_BP.Key_BP_C|Getph_key (Variables|Default|GetKey))))))
  (Transformation|SetActorRelativeTransform _key_2 (Variables|Default|GetKeySnapPoint) false true)
  ;[1 0.9952 0.3837] Turn off gravity and physics while in lock, turn them on when not.
  (Variables|Default|SetKeyGravityEnabled (Variables|/Game/UVRFProject/Framework/Hands/Grabable.Grabable_C|GetGravityEnabled _grabable))
  (Variables|/Game/UVRFProject/Framework/Hands/Grabable.Grabable_C|SetGravityEnabled _grabable false)
  (Variables|Default|SetKeySimulationPhysics (Variables|/Game/UVRFProject/Framework/Hands/Grabable.Grabable_C|GetSimulationPhysics _grabable))
  (Variables|/Game/UVRFProject/Framework/Hands/Grabable.Grabable_C|SetSimulationPhysics _grabable false)
  (Physics|SetSimulatePhysics _ph_key false)
  (Physics|SetEnableGravity _ph_key false))

(fn KeyInsertedTick
  (bind _key (Variables|Default|GetKey))
  (bind _ph_key (Variables|/Game/HarlowsWallpaper/Interaction/Interactable_keys_locks/Key_BP.Key_BP_C|Getph_key _key))
  (bind _returnvalue (Transformation|GetRelativeTransform _ph_key))
  (if (Variables|Default|GetAreProperAxesRestricted)
    _
    (else
      (Default|SetRestrictedAxes (Variables|/Game/HarlowsWallpaper/Interaction/Interactable_keys_locks/Key_BP.Key_BP_C|GetGrabable (Variables|Default|GetKey)) false false true true true true true true true true true true)
      (Variables|Default|SetAreProperAxesRestricted true)))
  ;[0.2868 1 0.9701] Check if leaving state
  (if (>= (.x (.location _returnvalue)) (Variables|LockPositionVars|GetKeyInserted_PullOutDistance)) ; if pulled out
    (Variables|Default|SetLockState "NewEnumerator4")
    (Variables|Default|SetAreProperAxesRestricted false)
    (CallFunction|RemoveKey)
    (elif (<= (.x (.location _returnvalue)) (Variables|LockPositionVars|GetKeyInserted_PushInDistance)) ; If pushed all the way in
      (Variables|Default|SetLockState "NewEnumerator1")
      (Variables|Default|SetAreProperAxesRestricted false)
      (Transformation|SetActorRelativeLocation (Variables|Default|GetKey) (Math|Vector|MakeVector (Variables|LockPositionVars|GetKeyInserted_PushInDistance) (.y (.location _returnvalue)) (.z (.location _returnvalue)))))))

(fn NoKeyTick)

(fn KeyFullyInsertedTick
  (bind _key (Variables|Default|GetKey))
  (bind _ph_key (Variables|/Game/HarlowsWallpaper/Interaction/Interactable_keys_locks/Key_BP.Key_BP_C|Getph_key _key))
  (bind _returnvalue (Transformation|GetRelativeTransform _ph_key))
  (if (Variables|Default|GetAreProperAxesRestricted)
    _
    (else
      (Default|SetRestrictedAxes (Variables|/Game/HarlowsWallpaper/Interaction/Interactable_keys_locks/Key_BP.Key_BP_C|GetGrabable (Variables|Default|GetKey)) false true true true true true true (Utilities|Enum|NotEqual(Enum) (Variables|Default|GetLock_Key_Id) (Variables|/Game/HarlowsWallpaper/Interaction/Interactable_keys_locks/Key_BP.Key_BP_C|GetLock_Key_ID (Variables|Default|GetKey))) true true true true)
      (Variables|Default|SetAreProperAxesRestricted true)))
  ;[0.2868 1 0.9701] Check if leaving state
  (if (>= (.x (.location _returnvalue)) (Variables|LockPositionVars|GetFullInsertion_PullOutDistance)) ; if pulled out
    (Variables|Default|SetLockState "NewEnumerator0")
    (Variables|Default|SetAreProperAxesRestricted false)
    (elif (Math|Float|InRange(Float) (Class|KismetMathLibrary|ClampAxis (.roll (.rotation _returnvalue))) (Class|KismetMathLibrary|ClampAxis (Variables|LockPositionVars|GetFullInsertion_RotateMin)) (Class|KismetMathLibrary|ClampAxis (Variables|LockPositionVars|GetFullInsertion_RotateMax))) ; If rotated enough to change state
      (Variables|Default|SetLockState "NewEnumerator2")
      (Variables|Default|SetAreProperAxesRestricted false))))

(fn KeyBeginsRotationTick
  (bind _key (Variables|Default|GetKey))
  (bind _ph_key (Variables|/Game/HarlowsWallpaper/Interaction/Interactable_keys_locks/Key_BP.Key_BP_C|Getph_key _key))
  (bind _returnvalue (Transformation|GetRelativeTransform _ph_key))
  (if (Variables|Default|GetAreProperAxesRestricted)
    _
    (else
      (Default|SetRestrictedAxes (Variables|/Game/HarlowsWallpaper/Interaction/Interactable_keys_locks/Key_BP.Key_BP_C|GetGrabable (Variables|Default|GetKey)) true true true true true true false false true true true true)
      (Variables|Default|SetAreProperAxesRestricted true)))
  ;[0.2868 1 0.9701] Check if leaving state
  (if (or (Math|Float|InRange(Float) (Class|KismetMathLibrary|ClampAxis (.roll (.rotation _returnvalue))) (Class|KismetMathLibrary|ClampAxis (Variables|LockPositionVars|GetBeginRotation_ReturnRotationMax)) 3.6e+02) (Math|Float|InRange(Float) (Class|KismetMathLibrary|ClampAxis (.roll (.rotation _returnvalue))) 0.0 (Class|KismetMathLibrary|ClampAxis (Variables|LockPositionVars|GetBeginRotation_ReturnRotationMin)))) ; Rotated back to hole alignment
    (Variables|Default|SetLockState "NewEnumerator1")
    (Variables|Default|SetAreProperAxesRestricted false)
    (Transformation|SetActorRelativeRotation (Variables|Default|GetKey)) ; Align key with hole before going to inserted state
    (elif (Math|Float|InRange(Float) (Class|KismetMathLibrary|ClampAxis (.roll (.rotation _returnvalue))) (Class|KismetMathLibrary|ClampAxis (Variables|LockPositionVars|GetBeginRotation_UnlockRotationMin)) (Class|KismetMathLibrary|ClampAxis (Variables|LockPositionVars|GetBeginRotation_UnlockRotationMax))) ; Rotated to unlock
      (Variables|Default|SetLockState "NewEnumerator3")
      (Variables|Default|SetAreProperAxesRestricted false)
      (Transformation|SetActorRelativeRotation (Variables|Default|GetKey) "0, 0,270.000000") ; Align key with hole before going to inserted state
    )))

(fn KeyFullyRotatedTick
  (if (Variables|Default|GetAreProperAxesRestricted)
    _
    (else
      (Default|SetRestrictedAxes (Variables|/Game/HarlowsWallpaper/Interaction/Interactable_keys_locks/Key_BP.Key_BP_C|GetGrabable (Variables|Default|GetKey)) true true true true true true false true true true true true)
      (Variables|Default|SetAreProperAxesRestricted true)))
  ;[0.2868 1 0.9701] Check if leaving state
  (if (Math|Float|InRange(Float) (Class|KismetMathLibrary|ClampAxis (.roll (.rotation (Transformation|GetRelativeTransform (Variables|/Game/HarlowsWallpaper/Interaction/Interactable_keys_locks/Key_BP.Key_BP_C|Getph_key (Variables|Default|GetKey)))))) (Class|KismetMathLibrary|ClampAxis (Variables|LockPositionVars|GetFullyRotated_ReturnRotationMin)) (Class|KismetMathLibrary|ClampAxis (Variables|LockPositionVars|GetFullyRotated_ReturnRotationMax))) ; if pulled out
    (Variables|Default|SetLockState "NewEnumerator2")
    (Variables|Default|SetAreProperAxesRestricted false)
    (elif (and (Variables|Default|GetisLocked) (Utilities|Enum|Equal(Enum) (Variables|Default|GetLock_Key_Id) (Variables|/Game/HarlowsWallpaper/Interaction/Interactable_keys_locks/Key_BP.Key_BP_C|GetLock_Key_ID (Variables|Default|GetKey)))) ; If locked, unlock
      (CallFunction|Unlock))))

(fn RemoveKey
  (bind _key (Variables|Default|GetKey))
  (bind _key_2 (Variables|Default|GetKey))
  (bind _grabable (Variables|/Game/HarlowsWallpaper/Interaction/Interactable_keys_locks/Key_BP.Key_BP_C|GetGrabable _key_2))
  (bind _grabable_2 (Variables|/Game/HarlowsWallpaper/Interaction/Interactable_keys_locks/Key_BP.Key_BP_C|GetGrabable _key))
  (Development|PrintString "Removing key")
  (if (== (Transformation|GetAttachParent (Variables|/Game/HarlowsWallpaper/Interaction/Interactable_keys_locks/Key_BP.Key_BP_C|Getph_key _key_2)) self)
    (Transformation|DetachFromActor _key_2 "KeepWorld" "KeepWorld" "KeepWorld"))
  (Variables|Default|SetKeyholeOpen true)
  (Default|SetRestrictedAxes _grabable false false false false false false false false false false false false)
  (Utilities|IsValid (Variables|/Game/UVRFProject/Framework/Hands/Grabable.Grabable_C|GetHand _grabable) ; Do not call snap if the key is not held
    (:Is%20Valid
      _)
    (:Is%20Not%20Valid
      _))
  (Variables|/Game/UVRFProject/Framework/Hands/Grabable.Grabable_C|SetGravityEnabled _grabable_2 (Variables|Default|GetKeyGravityEnabled))
  (Variables|/Game/UVRFProject/Framework/Hands/Grabable.Grabable_C|SetSimulationPhysics _grabable_2 (Variables|Default|GetKeySimulationPhysics))
  (Default|SnaptoHoldPos _grabable))