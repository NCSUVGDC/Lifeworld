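; VR player pawn for Harlow's Wallpaper, with a non-VR fallback.
; On BeginPlay it creates the sound manager and gender selection widget, then detects the headset to spawn Touch or Vive controllers and offset hands on the trackers.
; Once a trigger enables it, Tick exaggerates real walking by offsetting the actor with scaled horizontal HMD movement.
; It also plays random gendered voice lines by event type and provides controller, laser and debug-log helpers.
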(event EventBeginPlay
  (bind _returnvalue (Game|ConstructObjectfromClass "/Game/HarlowsWallpaper/Environment/sounds/SoundManager.SoundManager_C" self))
  (Variables|Sound|SetsoundManagerRef _returnvalue)
  (UserInterface|CreateWidget "/Game/HarlowsWallpaper/UI/GenderSelection.GenderSelection_C" (Game|GetPlayerController 0))
  (Utilities|FlowControl|Sequence
    (:then_0
      ;[1 1 1] UVRF-Framework-specific logic
      (switch name (Class|HeadMountedDisplayFunctionLibrary|GetHMDDeviceName)
        (:Default
          (Setup|SetupNonVR))
        (:OculusRift
          (Setup|SetupRift :!label _label))
        (:SteamVR
          (Setup|SetupVive))
        (:OculusHMD
          (goto _label))))))

(event EventTick
  (params (DeltaSeconds :type Float%20%28single-precision%29))
  (CallFunction|ApplyMovementScaling))

(event EventGetVoices
  (params (eventType :type String))
  (bind _femalevoices (Variables|Sound|GetfemaleVoices))
  (bind _malevoices (Variables|Sound|GetmaleVoices))
  (bind _audio (Variables|Default|GetAudio))
  (bind (_general _obsession _fallingfloor) (Utilities|Struct|BreakfemaleVoiceArrayStruct _femalevoices))
  (bind (_general_2 _obsession_2 _fallingfloor_2) (Utilities|Struct|BreakmaleVoiceArrayStruct _malevoices))
  (if (Variables|Default|GetvoicesActivated)
    (switch string (Variables|Sound|GetchosenGender)
      (:Male
        (switch string eventType
          (:General
            (Variables|Sound|SetvoiceArray _general_2))
          (:Obsession
            (Variables|Sound|SetvoiceArray _obsession_2))
          (:FallingFloor
            (Variables|Sound|SetvoiceArray _fallingfloor_2))))
      (:Female
        (switch string eventType
          (:General
            (Variables|Sound|SetvoiceArray _general))
          (:Obsession
            (Variables|Sound|SetvoiceArray _obsession))
          (:FallingFloor
            (Variables|Sound|SetvoiceArray _fallingfloor)))))
    (Audio|Components|Audio|SetSound _audio (Utilities|Array|Get(acopy) (Variables|Sound|GetvoiceArray) (Math|Random|RandomIntegerinRange 0 (Utilities|Array|LastIndex (Variables|Sound|GetvoiceArray)))))
    (Audio|Components|Audio|Play _audio 0.0)))

(event Input|KeyboardEvents|MotionControllerLeftFaceButton1
  (params (Key :type Key%20Structure))
  ;[0.5481 1 0.2557] Increase/Decrease Movement Scaling
)

(event Input|KeyboardEvents|MotionControllerRightTrigger
  (params (Key :type Key%20Structure))
  ;[1 0.06219 0] Disable scaling until trigger is pulled
  (:Pressed
    (Variables|MovementScaling|SetMovement%20Scaling%20Enabled true)))

(event Input|KeyboardEvents|MotionControllerRightFaceButton1
  (params (Key :type Key%20Structure))
  ;[0.5481 1 0.2557] Increase/Decrease Movement Scaling
)

(event Input|KeyboardEvents|MotionControllerLeftTrigger
  (params (Key :type Key%20Structure))
  ;[1 0.06219 0] Disable scaling until trigger is pulled
  (:Pressed
    (Variables|MovementScaling|SetMovement%20Scaling%20Enabled true)))

(fn ConstructionScript)

(fn SetupRift
  (bind _returnvalue (Transformation|GetActorTransform))
  (bind _returnvalue_2 (Game|SpawnActorfromClass "/Game/UVRFProject/Framework/Controllers/Touch/TouchController.TouchController_C" _returnvalue "Undefined" 0 0))
  (bind _output_get (Variables|Default|SetLeftController _returnvalue_2))
  (Transformation|AttachComponentToComponent _output_get (Variables|Default|GetLeftTracker) "None" "SnapToTarget" "SnapToTarget" "SnapToTarget" true)
  (Default|SetControllerType _output_get "Left")
  (bind _returnvalue_3 (Game|SpawnActorfromClass "/Game/UVRFProject/Framework/Controllers/Touch/TouchController.TouchController_C" _returnvalue "Undefined" 0 0))
  (bind _output_get_2 (Variables|Default|SetRightController _returnvalue_3))
  (Transformation|AttachComponentToComponent _output_get_2 (Variables|Default|GetRightTracker) "None" "SnapToTarget" "SnapToTarget" "SnapToTarget" true)
  (Default|SetControllerType _output_get_2 "Right")
  (Setup|SpawnHands)
  (Default|ApplyControllerOffset (Variables|Default|GetLeftHand) "8.500000,1.000000,-2.500000" "-20.000000,-100.000000,-90.000000")
  (Default|ApplyControllerOffset (Variables|Default|GetRightHand) "8.500000,1.000000,-2.500000" "-20.000000,-100.000000,-90.000000")
  (CallFunction|ShowController true)
  (Class|HeadMountedDisplayFunctionLibrary|SetTrackingOrigin "Floor"))

(fn SetupVive
  (bind _returnvalue (Transformation|GetActorTransform))
  (bind _returnvalue_2 (Game|SpawnActorfromClass "/Game/UVRFProject/Framework/Controllers/HTCVive/ViveWand.ViveWand_C" _returnvalue "Undefined" 0 0))
  (bind _output_get (Variables|Default|SetLeftController _returnvalue_2))
  (Transformation|AttachComponentToComponent _output_get (Variables|Default|GetLeftTracker) "None" "SnapToTarget" "SnapToTarget" "SnapToTarget" true)
  (Default|SetControllerType _output_get "Left")
  (bind _returnvalue_3 (Game|SpawnActorfromClass "/Game/UVRFProject/Framework/Controllers/HTCVive/ViveWand.ViveWand_C" _returnvalue "Undefined" 0 0))
  (bind _output_get_2 (Variables|Default|SetRightController _returnvalue_3))
  (Transformation|AttachComponentToComponent _output_get_2 (Variables|Default|GetRightTracker) "None" "SnapToTarget" "SnapToTarget" "SnapToTarget" true)
  (Default|SetControllerType _output_get_2 "Right")
  (Setup|SpawnHands)
  (Default|ApplyControllerOffset (Variables|Default|GetLeftHand) "2.500000,2.000000,-8.000000" "-10.000000,-100.000000,-50.000000")
  (Default|ApplyControllerOffset (Variables|Default|GetRightHand) "2.500000,2.000000,-8.000000" "-10.000000,-100.000000,-50.000000")
  (CallFunction|ShowController true)
  (Class|HeadMountedDisplayFunctionLibrary|SetTrackingOrigin "Floor"))

(fn SpawnHands
  (bind _output_get (LocalVariables|SetHand%20Transform (Transformation|GetActorTransform)))
  ;[1 1 1] Spawn Hand Actors
  (bind _returnvalue (Game|SpawnActorfromClass "/Game/UVRFProject/Framework/Hands/HandBP.HandBP_C" _output_get "Undefined" 0 "Left" self 0))
  (bind _output_get_2 (Variables|Default|SetLeftHand _returnvalue))
  (Default|Setup _output_get_2)
  (bind _returnvalue_2 (Game|SpawnActorfromClass "/Game/UVRFProject/Framework/Hands/HandBP.HandBP_C" (LocalVariables|GetHand%20Transform) "Undefined" 0 "Right" self 0))
  (bind _output_get_3 (Variables|Default|SetRightHand _returnvalue_2))
  (Default|Setup _output_get_3)
  ;[1 1 1] Attach hands/invert left hand model
  (Transformation|AttachComponentToComponent (Variables|Default|GetLeftHand) (Variables|Default|GetLeftTracker) "None" "SnapToTarget" "SnapToTarget" "SnapToTarget" true)
  (Transformation|AttachComponentToComponent (Variables|Default|GetRightHand) (Variables|Default|GetRightTracker) "None" "SnapToTarget" "SnapToTarget" "SnapToTarget" true)
  (Transformation|SetActorScale3D (Variables|Default|GetLeftHand) "1.000000,-1.000000,1.000000")
  ;[1 1 1] Only setup VR controllers if in VR mode (otherwise they won't exist anyway)
  (if (not (Variables|Default|GetNonVR%20Mode))
    (Variables|/Game/UVRFProject/Framework/Controllers/MotionControllerBase.MotionControllerBase_C|SetHandActor (Variables|Default|GetLeftController) (Variables|Default|GetLeftHand))
    (Variables|/Game/UVRFProject/Framework/Controllers/MotionControllerBase.MotionControllerBase_C|SetHandActor (Variables|Default|GetRightController) (Variables|Default|GetRightHand))))

(fn ShowController
  (params (Hide%20Contollers :type Boolean))
  (Rendering|SetActorHiddenInGame (Variables|Default|GetRightController) Hide%20Contollers))

(fn GetCameraYaw
  (return (.Yaw (Math|Rotator|BreakRotator (Transformation|GetWorldRotation (Variables|Default|GetPrimaryCam))))))

(fn ToggleController
  (CallFunction|ShowController (not (Variables|/Script/Engine.Actor|GetbHidden (Variables|Default|GetLeftController)))))

(fn ToggleLaser
  (bind _righthand (Variables|Default|GetRightHand))
  (bind _lefthand (Variables|Default|GetLeftHand))
  (if (Default|IsLaserActive _righthand)
    (Default|DeactivateLaser _righthand)
    (else
      (Default|ActivateLaser _righthand)))
  (if (Default|IsLaserActive _lefthand)
    (Default|DeactivateLaser _lefthand)
    (else
      (Default|ActivateLaser _lefthand))))

(fn ApplyMovementScaling
  (bind _movement_scaling (Variables|MovementScaling|GetMovement%20Scaling))
  (bind _returnvalue (* _movement_scaling -1.0))
  ;[1 1 1] Allow scaling to be toggled
  (if (Variables|MovementScaling|GetMovement%20Scaling%20Enabled)
    (Utilities|FlowControl|Sequence
      (:then_0
        ;[1 0.3441 0.4541] Ignore first tick
        (if (Math|Vector|NotEqual(Vector) (Variables|MovementScaling|GetHMD%20Location%20%28End%20of%20Tick%29) "0, 0, 0" 0.001)
          ;[1 0.8207 0.3953] Get True Motion from Headset
          (bind _output_get (LocalVariables|SetReal%20HMD%20Delta (- (Variables|MovementScaling|GetHMD%20Location%20%28End%20of%20Tick%29) (Variables|/Script/Engine.SceneComponent|GetRelativeLocation (Variables|Default|GetPrimaryCam)))))
          ;[1 0.7701 0.3623] Scale True Motion
          (bind _output_get_2 (LocalVariables|SetScaled%20HMD%20Delta (* _output_get (Math|Vector|MakeVector _returnvalue _returnvalue 0.0))))
          ;[0.2047 0.1752 1] Apply Exaggerated Motion
          (Transformation|AddActorLocalOffset _output_get_2 false false)))
      (:then_1
        ;[0.3112 0.7663 1] Lastly, Save the HMD Location
        (Variables|MovementScaling|SetHMD%20Location%20%28End%20of%20Tick%29 (Variables|/Script/Engine.SceneComponent|GetRelativeLocation (Variables|Default|GetPrimaryCam)))))))

(fn AddDebugMessage
  (params (Message :type Text) (Lifespan :type Float%20%28single-precision%29) (Verbosity :type DebugVerbosity%20Enum :default "NewEnumerator4"))
  (bind _asui_debug_log (Utilities|Casting|CastToUI_DebugLog (UserInterface|GetUserWidgetObject (Variables|Default|GetWidget))))
  (Default|AddMessage _asui_debug_log Message Verbosity Lifespan))

(fn SetupNonVR
  (Variables|Default|SetNonVR%20Mode true)
  (Setup|SpawnHands))