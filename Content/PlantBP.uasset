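; PlantBP tracks how long the plant takes to fully ignite, so that the same period can serve as its burnout time.
; A 90-second timer on an empty function acts as a stopwatch from BeginPlay, while Tick re-queries Flammable-tagged actors.
; While Burning, GetBurnShit waits until none remain, converts elapsed time into 0.05-second iterations for the passed object, then clears Burning once over a second has elapsed.
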(event Custom|SetBurning
  (Variables|Default|SetBurning? true))

(event Custom|SetBurnout
  (Variables|Default|SetBurning? false))

(event Custom|GetBurnShit
  (params (NewParam :type Flame%20Leaf%20Object%20Reference))
  (bind _returnvalue (Class|KismetSystemLibrary|GetTimerRemainingTime 0 "NewFunction_0"))
  ;[1 1 1] This basically watches to see how long it takes the plant to fully ignite so that we can use that time period as the time it takes to burn out
  (if (Variables|Default|GetBurning?)
    (if (== (Utilities|Array|Length (stale EventTick _outactors)) 0)
      (bind _output_get (Variables|/Game/HarlowsWallpaper/FlameLeaf.FlameLeaf_C|SetBurnIterations NewParam (Math|Float|Round (/ (- 9e+01 _returnvalue) 0.05))))
      (Default|IterationSet NewParam _output_get)
      (if (< _returnvalue 89.0)
        (CallFunction|SetBurnout)))))

(event EventBeginPlay
  ;[1 1 1] Start with an array of all items with Flammable tag
  (Utilities|Time|SetTimerbyFunctionName 0 "NewFunction_0" 9e+01)
  (bind _outactors (Actor|GetAllActorswithTag "Flammable"))
  (for _array_element _outactors
    (Utilities|Array|Add (Variables|Default|GetInflammableArray) _array_element)))

(event EventTick
  (params (DeltaSeconds :type Float%20%28single-precision%29))
  ;[1 1 1] This basically watches to see how long it takes the plant to fully ignite so that we can use that time period as the time it takes to burn out
  (bind _outactors (Actor|GetAllActorswithTag "Flammable")))

(fn ConstructionScript)

(fn NewFunction0)